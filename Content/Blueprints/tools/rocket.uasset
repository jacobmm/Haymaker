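; Rocket projectile that speeds up from a slow start, then homes back toward its Papa actor.
; Each tick below a speed threshold nudges velocity along +X; reaching it leads to a four-second delay before setting the Return flag.
; The ProjectileMovement component then homes on Papa's root component with randomized acceleration.
; The construction script seeds its velocity and initial speed from variables.
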(event `self.ReceiveTick`
  (params (DeltaSeconds :type "Float (single-precision)"))
  (bind _projectilemovement (`self.ProjectileMovement`))
  (bind _projectilemovement_2 (`self.ProjectileMovement`))
  (bind _velocity (`MovementComponent.Velocity` _projectilemovement_2))
  (if (`self.return`)
    _
    (elif (< (`KismetMathLibrary.VSize` _velocity) 50.0)
      (set `MovementComponent.Velocity` (- _velocity (-1.0 0.0 0.0)) _projectilemovement_2)
      (else
        (`KismetSystemLibrary.Delay` 4.0)
        (set `self.return` true)
        (set `ProjectileMovementComponent.HomingTargetComponent` (`self.K2_GetRootComponent` (`self.papa`)) _projectilemovement)
        (set `ProjectileMovementComponent.bIsHomingProjectile` true _projectilemovement)
        (set `ProjectileMovementComponent.HomingAccelerationMagnitude` (`KismetMathLibrary.RandomFloatInRange` 400.0 800.0) _projectilemovement)))))

(event `self.ReceiveActorBeginOverlap`
  (params (OtherActor :type "Actor Object Reference")))

(fn `UserConstructionScript`
  (bind _projectilemovement (`self.ProjectileMovement`))
  (set `MovementComponent.Velocity` (`self.myVelocity`) _projectilemovement)
  (set `ProjectileMovementComponent.InitialSpeed` (`self.mySpeed`) _projectilemovement))