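; Laser beam actor that ends its particle beam on whatever surface lies in front of it.
; Each Tick it line-traces on Visibility along the beam component's forward vector and sets the beam target to the impact point.
; It also spawns a new spark emitter every frame, oriented to the hit normal and nudged along world X, without checking whether the trace hit.
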(event `self.ReceiveBeginPlay`)

(event `self.ReceiveActorBeginOverlap`
  (params (OtherActor :type "Actor Object Reference")))

(event `self.ReceiveTick`
  (params (DeltaSeconds :type "Float (single-precision)"))
  (bind _laserbeam (`self.laserBeam`))
  (bind _returnvalue (`SceneComponent.K2_GetComponentLocation` _laserbeam))
  (bind _outhit (`KismetSystemLibrary.LineTraceSingle` _returnvalue (+ _returnvalue (* (`KismetMathLibrary.GetForwardVector` (`SceneComponent.K2_GetComponentRotation` _laserbeam)) 3000.0)) "TraceTypeQuery1"))
  (bind (_bblockinghit _binitialoverlap _time _location _impactpoint _normal) (`GameplayStatics.BreakHitResult` _outhit))
  (`ParticleSystemComponent.SetBeamTargetPoint` (`self.laserBeam`) 0 _impactpoint 0)
  (`GameplayStatics.SpawnEmitterAtLocation` "/Game/StarterContent/Particles/P_Sparks.P_Sparks" (+ _impactpoint (-5.0 0.0 0.0)) (`KismetMathLibrary.Conv_VectorToRotator` _normal)))

(fn `UserConstructionScript`)