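; Construction-script tool that tiles a floor with rows of rock meshes, with counts derived from FloorEnd.
; Each row's seeded random widths are normalized to a common length, then accumulated by half-widths into center positions for the scaled pieces.
; Pieces get a seeded yaw, while a random MultiGate picks one of four meshes and tints, with unseeded roughness on dynamic material instances.
; An older grid-placement branch remains unconnected.
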(fn ConstructionScript
  (bind _floorend (Variables|Default|GetfloorEnd))
  (bind (_x _y) (Math|Vector|BreakVector _floorend))
  (bind _returnvalue (/ _y 256.0))
  (bind _returnvalue_2 (/ _x 256.0))
  (bind _returnvalue_3 (Math|Float|Floor _returnvalue_2))
  (bind _returnvalue_4 (Math|Float|Floor _returnvalue))
  (if (Math|Vector|NotEqual(Vector) (* (Variables|Default|GetfloorEnd) "1.000000,1.000000,0.000000") "0, 0, 0" 1e-06)
    (Variables|Default|SetnumOfRockLong _returnvalue_3)
    (Variables|Default|SetnumOfRockHigh _returnvalue_4)
    (Development|PrintString (Utilities|String|Append (Utilities|String|Append (Utilities|String|Append (Utilities|String|Append "( " (Utilities|String|ToString(Integer) _returnvalue_3)) ", ") (Utilities|String|ToString(Integer) _returnvalue_4)) " )")))
  (for _index (range 0 (+ (Variables|Default|GetnumOfRockHigh) 1))
    (Variables|Default|SetheightPosition (* _index (Variables|Default|GetheightOfRock)))
    (bind _randomnumbers (CallFunction|CreateRandomArray (Variables|Default|GetminScale) (Variables|Default|GetmaxScale) (Variables|Default|GetnumOfRockLong) (Variables|Default|GetmyRandomStream)))
    (bind _scaledfloats (CallFunction|ScaleArray _randomnumbers (Math|Conversions|ToFloat(Integer) (Variables|Default|GetnumOfRockLong))))
    (Variables|Default|SetrockScaleValues _scaledfloats)
    (bind _scaledfloats_2 (CallFunction|ScaleArray _randomnumbers (* (Variables|Default|GetnumOfRockLong) (Variables|Default|GetlengthOfRock))))
    (bind _returnnewarray (CallFunction|FloorPosition _scaledfloats_2))
    (Variables|Default|SetrockPositionValues _returnnewarray)
    (for _index_2 (range 0 (- (Variables|Default|GetnumOfRockLong) 1))
      (bind _returnvalue_5 (AddComponent|AddStaticMeshComponent false (Math|Transform|MakeTransform (Math|Vector|MakeVector (Utilities|Array|Get(acopy) (Variables|Default|GetrockPositionValues) _index_2) (Variables|Default|GetheightPosition) 0.0) (Class|KismetMathLibrary|MakeRot 0.0 (* (Math|Conversions|ToFloat(Integer) (Math|Random|RandomIntegerinRangefromStream -1 1 (Variables|Default|GetmyRandomStream))) 9e+01) 0.0) (Math|Vector|MakeVector (Utilities|Array|Get(acopy) (Variables|Default|GetrockScaleValues) _index_2) 1.0 1.0))))
      ;[1 1 1] tinting and setup of materials
      (Utilities|FlowControl|MultiGate true true -1
        (:Out%200
          (bind _returnvalue_6 (Rendering|Material|CreateDynamicMaterialInstance _returnvalue_5 0 "/Game/artSource/materials/floor/floor_MI.floor_MI" :!class /Script/Engine.PrimitiveComponent))
          (Rendering|Material|SetVectorParameterValue _returnvalue_6 "floorColor" "(R=0.580000,G=0.540292,B=0.095700,A=0.000000)" :!class /Script/Engine.MaterialInstanceDynamic)
          (Rendering|Material|SetScalarParameterValue _returnvalue_6 "roughness" (Math|Random|RandomFloatinRange 6.5 12.1) :!class /Script/Engine.MaterialInstanceDynamic)
          (Components|StaticMesh|SetStaticMesh _returnvalue_5 "/Game/artSource/Meshes/floor/floorA.floorA"))
        (:Out%201
          (bind _returnvalue_7 (Rendering|Material|CreateDynamicMaterialInstance _returnvalue_5 0 "/Game/artSource/materials/floor/floor_MI.floor_MI" :!class /Script/Engine.PrimitiveComponent))
          (Rendering|Material|SetVectorParameterValue _returnvalue_7 "floorColor" "(R=0.580000,G=0.491212,B=0.095700,A=0.000000)" :!class /Script/Engine.MaterialInstanceDynamic)
          (Rendering|Material|SetScalarParameterValue _returnvalue_7 "roughness" (Math|Random|RandomFloatinRange 6.5 12.1) :!class /Script/Engine.MaterialInstanceDynamic)
          (Components|StaticMesh|SetStaticMesh _returnvalue_5 "/Game/artSource/Meshes/floor/floorB.floorB"))
        (:Out%202
          (bind _returnvalue_8 (Rendering|Material|CreateDynamicMaterialInstance _returnvalue_5 0 "/Game/artSource/materials/floor/floor_MI.floor_MI" :!class /Script/Engine.PrimitiveComponent))
          (Rendering|Material|SetVectorParameterValue _returnvalue_8 "floorColor" "(R=0.571928,G=0.580000,B=0.095700,A=0.000000)" :!class /Script/Engine.MaterialInstanceDynamic)
          (Rendering|Material|SetScalarParameterValue _returnvalue_8 "roughness" (Math|Random|RandomFloatinRange 6.5 12.1) :!class /Script/Engine.MaterialInstanceDynamic)
          (Components|StaticMesh|SetStaticMesh _returnvalue_5 "/Game/artSource/Meshes/floor/floorC.floorC"))
        (:Out%203
          (bind _returnvalue_9 (Rendering|Material|CreateDynamicMaterialInstance _returnvalue_5 0 "/Game/artSource/materials/floor/floor_MI.floor_MI" :!class /Script/Engine.PrimitiveComponent))
          (Rendering|Material|SetVectorParameterValue _returnvalue_9 "floorColor" "(R=0.489000,G=0.439766,B=0.066993,A=0.000000)" :!class /Script/Engine.MaterialInstanceDynamic)
          (Rendering|Material|SetScalarParameterValue _returnvalue_9 "roughness" (Math|Random|RandomFloatinRange 6.5 12.1) :!class /Script/Engine.MaterialInstanceDynamic)
          (Components|StaticMesh|SetStaticMesh _returnvalue_5 "/Game/artSource/Meshes/floor/floorD.floorD"))))))

(fn CreateRandomArray
  (params (minValue :type Float%20%28single-precision%29) (maxValue :type Float%20%28single-precision%29) (numElements :type Integer) (randomStream :type Random%20Stream%20Structure%20%28by%20ref%29))
  (for _index (range 0 (- numElements 1))
    (Utilities|Array|Add (LocalVariables|GetReturnArray) (Math|Random|RandomFloatinRangefromStream minValue maxValue randomStream)))
  (return (LocalVariables|GetReturnArray)))

(fn MyPrintArray
  (params (inArray :type Array%20of%20Floats%20%28single-precision%29))
  (Development|PrintString "----------------------------------------------------------")
  (for _array_element inArray
    (Development|PrintString (Utilities|String|ToString(Float) _array_element)))
  (Development|PrintString "*************************************************************"))

(fn ScaleArray
  (params (inputRandomArray :type Array%20of%20Floats%20%28single-precision%29) (targetSum :type Float%20%28single-precision%29))
  (LocalVariables|SetinputSum 0.0)
  ;[1 1 1] calc current total
  (for _array_element inputRandomArray
    (LocalVariables|SetinputSum (+ (LocalVariables|GetinputSum) _array_element)))
  ;[1 1 1] calc scale factor
  (LocalVariables|SetScaleFactor (/ targetSum (LocalVariables|GetinputSum)))
  ;[1 1 1] scale the array
  (for _array_element_2 inputRandomArray
    (Utilities|Array|Add (LocalVariables|GetReturnArray) (* _array_element_2 (LocalVariables|GetScaleFactor))))
  (return (LocalVariables|GetReturnArray)))

(fn FloorPosition
  (params (floorSize :type Array%20of%20Floats%20%28single-precision%29))
  (LocalVariables|SetcurrentTotal 0.0)
  (LocalVariables|SetpreviousElement 0.0)
  (for _array_element floorSize
    (Utilities|FlowControl|Sequence
      (:then_0
        ;[1 1 1] calculate new total
        (LocalVariables|SetnewElement _array_element)
        (LocalVariables|SetnewTotal (|oldTotal+0.5*(newElement+prevElement) (LocalVariables|GetcurrentTotal) (LocalVariables|GetnewElement) (LocalVariables|GetpreviousElement)))
        (Utilities|Array|Add (LocalVariables|GetreturnArray) (LocalVariables|GetnewTotal)))
      (:then_1
        ;[1 1 1] prep next round of loop
        (LocalVariables|SetcurrentTotal (LocalVariables|GetnewTotal))
        (LocalVariables|SetpreviousElement (LocalVariables|GetnewElement)))))
  (return (LocalVariables|GetreturnArray)))