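; Toggleable door Blueprint that slides its Mover 310 units down to open and back up to close.
; Trigger flip-flops open and close, and switch events call them directly, driving a timeline that lerps from the current position toward either end.
; A timed trigger uses MoveComponentTo instead, and ResetObject snaps the door shut.
; The construction script configures door and indicator meshes, a dynamic color/opacity material, name tag and text label.
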(event `/Game/Blueprints/haymkaerBP/timerInteraction_BPI.resetObject`
  (`|ExecutionSequence`
    (:`then_0`
      (goto _label_2 :!via `Stop`))
    (:`then_1`
      (bind _output_get (set `self.doorLocation` (`self.locationA`)))
      (`SceneComponent.K2_SetRelativeLocation` (`self.mover`) _output_get false false))))

(event `self.ReceiveBeginPlay`
  (bind _relativelocation (`SceneComponent.RelativeLocation` (`self.mover`)))
  (`TimelineComponent.Stop` (`self.doorOpen`))
  (set `self.locationA` _relativelocation)
  (set `self.locationB` (- _relativelocation (0.0 0.0 310.0)))
  (`TimelineComponent.SetPlayRate` (`self.doorOpen`) (`self.playRate`))
  (set `self.doorLocation` (`SceneComponent.RelativeLocation` (`self.mover`))))

(event `openDoor`
  (bind _mover (`self.mover`))
  ;[1 1 1] Comment
  (`TimelineComponent.SetPlayRate` (`self.doorOpen`) (`self.playRate`))
  (bind (_direction _alpha) (`Timeline|doorOpen` :!label _label)
    (:`Update`
      (switch `ETimelineDirection` _direction
        (:`Forward`
          (`SceneComponent.K2_SetRelativeLocation` _mover (`KismetMathLibrary.VLerp` (`SceneComponent.RelativeLocation` (`self.mover`)) (`self.locationB`) _alpha) false false))
        (:`Backward`
          (`SceneComponent.K2_SetRelativeLocation` _mover (`KismetMathLibrary.VLerp` (`SceneComponent.RelativeLocation` (`self.mover`)) (`self.locationA`) _alpha) false false))))))

(event `closeDoor`
  ;[1 1 1] Comment
  (`TimelineComponent.SetPlayRate` (`self.doorOpen`) (`self.playRate`))
  (goto _label :!via `Reverse`))

(event `timedTrigger`
  (params (timedTrigger :type "Float (double-precision)"))
  ;[1 1 1] Comment
  (set `self.openDoorTime` timedTrigger)
  (`KismetSystemLibrary.MoveComponentTo` (`self.mover`) (`self.locationB`) (struct) true true (`self.playRate`))
  (`KismetSystemLibrary.MoveComponentTo` (`self.mover`) (`self.locationA`) (struct) true true (`self.openDoorTime`) :!label _label_2))

(event `trigger`
  ;[1 1 1] Comment
  (`/Engine/EditorBlueprintResources/StandardMacros.FlipFlop`
    (:`A`
      (`self.openDoor`))
    (:`B`
      (`self.closeDoor`))))

(event `openWithSwitch`
  ;[1 1 1] Comment
  (`self.openDoor`))

(event `closeWithSwitch`
  ;[1 1 1] Comment
  (`self.closeDoor`))

(fn `UserConstructionScript`
  (bind _textrender3 (`self.TextRender3`))
  (bind _doorindicator (`self.doorIndicator`))
  (bind _staticmesh (`self.StaticMesh`))
  (`StaticMeshComponent.SetStaticMesh` _staticmesh (`self.doorMesh`))
  (`SceneComponent.K2_SetRelativeTransform` _staticmesh (`self.door mesh transform`) false false)
  (`StaticMeshComponent.SetStaticMesh` _doorindicator (`self.indicatorMesh`))
  (`SceneComponent.K2_SetRelativeTransform` _doorindicator (`self.indicatorTransform`) false false)
  (bind _returnvalue (`PrimitiveComponent.CreateDynamicMaterialInstance` (`self.StaticMesh`) 0 "/Game/artSource/materials/doorIndicator_M.doorIndicator_M"))
  (bind _output_get (set `self.indicatorMaterial` _returnvalue))
  (`MaterialInstanceDynamic.SetVectorParameterValue` _output_get "color" (`self.lockColor`))
  (`MaterialInstanceDynamic.SetScalarParameterValue` _output_get "activate" (`self.doorOpacity`))
  (`KismetArrayLibrary.Array_Set` (`self.Tags`) 0 (`self.door name`))
  (`SceneComponent.K2_SetRelativeLocationAndRotation` _textrender3 (`self.text location`) (`self.text Rotation`) false false)
  (`TextRenderComponent.K2_SetText` _textrender3 (`self.door Text`))
  (if (`self.attachIndicatorToDoor`)
    (`SceneComponent.K2_AttachTo` (`self.doorIndicator`) (`self.StaticMesh`) "None" "KeepWorldPosition" true)))