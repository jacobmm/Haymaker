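; Level switch tool that lets the player cycle through selectable levels.
; Overlapping ActivateTrigger as MyCharacter enables use, and no end-overlap handler disables it.
; SwitchPress plays a sound, advances a wrapping LevelPick counter and maps it to the CurrentLevel enum on the player's character.
; Two helper functions rotate rings by fixed steps, but nothing in this Blueprint calls them.
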(event `self.ReceiveTick`
  (params (DeltaSeconds :type "Float (single-precision)")))

(event `/Game/Blueprints/tools/buttonInteraction_BPI.switchPress`
  (if (`self.canUse`)
    (`GameplayStatics.PlaySound2D` "/Game/artSource/sounds/levelSelect.levelSelect")
    (bind _output_get (set `self.levelPick` (+ (`self.levelPick`) 1)))
    (if (>= _output_get 17)
      (set `self.levelPick` 1))
    (bind _asmy_character (cast `/Game/Blueprints/MyCharacter` (`Controller.K2_GetPawn` (`GameplayStatics.GetPlayerController` 0))))
    (switch `int` (`self.levelPick`)
      (:`0`
        (set `/Game/Blueprints/MyCharacter.currentLevel` "NewEnumerator24" _asmy_character))
      (:`1`
        (set `/Game/Blueprints/MyCharacter.currentLevel` "NewEnumerator0" _asmy_character))
      (:`2`
        (set `/Game/Blueprints/MyCharacter.currentLevel` "NewEnumerator1" _asmy_character))
      (:`3`
        (set `/Game/Blueprints/MyCharacter.currentLevel` "NewEnumerator2" _asmy_character))
      (:`4`
        (set `/Game/Blueprints/MyCharacter.currentLevel` "NewEnumerator15" _asmy_character))
      (:`5`
        (set `/Game/Blueprints/MyCharacter.currentLevel` "NewEnumerator3" _asmy_character))
      (:`6`
        (set `/Game/Blueprints/MyCharacter.currentLevel` "NewEnumerator4" _asmy_character))
      (:`7`
        (set `/Game/Blueprints/MyCharacter.currentLevel` "NewEnumerator5" _asmy_character))
      (:`8`
        (set `/Game/Blueprints/MyCharacter.currentLevel` "NewEnumerator6" _asmy_character))
      (:`9`
        (set `/Game/Blueprints/MyCharacter.currentLevel` "NewEnumerator7" _asmy_character))
      (:`10`
        (set `/Game/Blueprints/MyCharacter.currentLevel` "NewEnumerator8" _asmy_character))
      (:`11`
        (set `/Game/Blueprints/MyCharacter.currentLevel` "NewEnumerator9" _asmy_character))
      (:`12`
        (set `/Game/Blueprints/MyCharacter.currentLevel` "NewEnumerator10" _asmy_character))
      (:`13`
        (set `/Game/Blueprints/MyCharacter.currentLevel` "NewEnumerator11" _asmy_character))
      (:`14`
        (set `/Game/Blueprints/MyCharacter.currentLevel` "NewEnumerator12" _asmy_character))
      (:`15`
        (set `/Game/Blueprints/MyCharacter.currentLevel` "NewEnumerator13" _asmy_character))
      (:`16`
        (set `/Game/Blueprints/MyCharacter.currentLevel` "NewEnumerator14" _asmy_character)))))

(event `self.activateTrigger.OnComponentBeginOverlap`
  (params (OtherActor :type "Actor Object Reference") (OtherComp :type "PrimitiveComponent Object Reference") (OtherBodyIndex :type Integer) (bFromSweep :type Boolean) (SweepResult :type "HitResult Structure (by ref)"))
  (bind _asmy_character (cast `/Game/Blueprints/MyCharacter` OtherActor))
  (if (== OtherActor _asmy_character)
    (set `self.canUse` true)
    (else
      (set `self.canUse` false))))

(fn `rotateRing1`
  (params (level1Ring :type "SceneComponent Object Reference"))
  (`SceneComponent.K2_SetRelativeRotation` level1Ring (`KismetMathLibrary.MakeRot` 0.0 (+ (.yaw (`SceneComponent.RelativeRotation` level1Ring)) -60.0)) false))

(fn `rotateRing2`
  (params (self2 :type "SceneComponent Object Reference"))
  (`SceneComponent.K2_SetRelativeRotation` self2 (`KismetMathLibrary.MakeRot` (.pitch (`SceneComponent.RelativeRotation` self2)) (.yaw (`SceneComponent.RelativeRotation` self2)) (+ (.roll (`SceneComponent.RelativeRotation` self2)) 70.0)) false))

(fn `UserConstructionScript`)