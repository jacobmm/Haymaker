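; Level portal actor built around an animated obelisk that sends the player's MyCharacter toward a new level.
; Overlapping the BallSeat sets OpenPortal on the obelisk_ABP anim instance and reveals the Plane; leaving it closes the portal and hides the Plane again.
; Overlapping the separate Box trigger calls LoadingNewLevel on the character, which handles the level change itself.
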(event `self.ReceiveTick`
  (params (DeltaSeconds :type "Float (single-precision)")))

(event `self.Box.OnComponentBeginOverlap`
  (params (OtherActor :type "Actor Object Reference") (OtherComp :type "PrimitiveComponent Object Reference") (OtherBodyIndex :type Integer) (bFromSweep :type Boolean) (SweepResult :type "HitResult Structure (by ref)"))
  ;[1 1 1] port to new level
  (bind _asmy_character (cast `/Game/Blueprints/MyCharacter` OtherActor))
  (if (== OtherActor _asmy_character)
    (`/Game/Blueprints/MyCharacter.loadingNewLevel` _asmy_character)))

(event `self.ballSeat.OnComponentBeginOverlap`
  (params (OtherActor :type "Actor Object Reference") (OtherComp :type "PrimitiveComponent Object Reference") (OtherBodyIndex :type Integer) (bFromSweep :type Boolean) (SweepResult :type "HitResult Structure (by ref)"))
  ;[1 1 1] spawn fake ball when I shoot obelisk
  (bind _asmy_character (cast `/Game/Blueprints/MyCharacter` OtherActor))
  (if (== OtherActor _asmy_character)
    (bind _asobelisk_abp (cast `/Game/artSource/animation/obelisk/obelisk_ABP` (`SkeletalMeshComponent.GetAnimInstance` (`self.obeliskRig`))))
    (set `/Game/artSource/animation/obelisk/obelisk_ABP.openPortal` true _asobelisk_abp)
    (`SceneComponent.SetHiddenInGame` (`self.plane`) false false)))

(event `self.ballSeat.OnComponentEndOverlap`
  (params (OtherActor :type "Actor Object Reference") (OtherComp :type "PrimitiveComponent Object Reference") (OtherBodyIndex :type Integer))
  (bind _asmy_character (cast `/Game/Blueprints/MyCharacter` OtherActor))
  (if (== OtherActor _asmy_character)
    (bind _asobelisk_abp (cast `/Game/artSource/animation/obelisk/obelisk_ABP` (`SkeletalMeshComponent.GetAnimInstance` (`self.obeliskRig`))))
    (set `/Game/artSource/animation/obelisk/obelisk_ABP.openPortal` false _asobelisk_abp)
    (`SceneComponent.SetHiddenInGame` (`self.plane`) true false)))

(fn `UserConstructionScript`)