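; A level start actor that sets the player's checkpoint and starts the level timer when the character overlaps it.
; On overlap it sends the SpawnPoint component's world location to MyCharacter as the level checkpoint, then messages the game state to start the timer.
; The construction script positions the spawn point and portal camera and scales the timer trigger from the actor's variables, so each placed instance can be configured.
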(event `self.ReceiveActorBeginOverlap`
  (params (OtherActor :type "Actor Object Reference"))
  (bind _asmy_character (cast `/Game/Blueprints/MyCharacter` OtherActor))
  (if (== _asmy_character OtherActor)
    (message `/Game/Blueprints/tools/timerInteraction_BPI.setLevelCheckpoint` _asmy_character (`SceneComponent.K2_GetComponentLocation` (`self.spawnPoint`)))
    (message `/Game/Blueprints/tools/timerInteraction_BPI.startTimer` (`GameplayStatics.GetGameState`))))

(fn `UserConstructionScript`
  (set `self.setLevel` (`self.setLevel`))
  (`SceneComponent.K2_SetRelativeLocation` (`self.spawnPoint`) (`self.levelSpawnPoint`) false)
  (`SceneComponent.SetRelativeScale3D` (`self.timerTrigger`) (`self.triggerScale`))
  (`SceneComponent.K2_SetRelativeLocationAndRotation` (`self.portalCam`) (`self.camera position`) (`self.camera rotation`) false))