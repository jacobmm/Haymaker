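; Projectile actor with a collision sphere and a projectile movement component that can be switched into homing on a target.
; The construction script sets the movement's velocity and initial speed from its own variables.
; The toggleHoming event, given a valid target, homes on its root component with a fixed acceleration; it has no off branch.
; The sphere's hit event is empty, and an actor-destroy node sits unconnected.
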(event `self.Sphere.OnComponentHit`
  (params (OtherActor :type "Actor Object Reference") (OtherComp :type "PrimitiveComponent Object Reference") (NormalImpulse :type "Vector Structure") (Hit :type "HitResult Structure (by ref)")))

(event `toggleHoming`
  (params (target :type "Actor Object Reference"))
  (bind _projectilemovement (`self.ProjectileMovement`))
  (if (`KismetSystemLibrary.IsValid` target)
    (set `ProjectileMovementComponent.HomingTargetComponent` (`self.K2_GetRootComponent` target) _projectilemovement)
    (set `ProjectileMovementComponent.bIsHomingProjectile` true _projectilemovement)
    (set `ProjectileMovementComponent.HomingAccelerationMagnitude` 2000.0 _projectilemovement)))

(fn `UserConstructionScript`
  (bind _projectilemovement (`self.ProjectileMovement`))
  (set `MovementComponent.Velocity` (`self.myVelocity`) _projectilemovement)
  (set `ProjectileMovementComponent.InitialSpeed` (`self.mySpeed`) _projectilemovement))