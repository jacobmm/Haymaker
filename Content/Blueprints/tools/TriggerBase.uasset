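; Hit-activated trigger base that operates ToggleDoor actors in either Toggle or Timer mode.
; Toggle flips the linked Door, while Timer triggers all doors tagged DoorName, then triggers them again after OpenTime.
; During the timer a ticking sound plays and Tick updates countdown text that faces the player's pawn.
; The construction script applies configurable mesh and collision settings and tints mesh and text with the linked Door's LockColor.
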(event `self.ReceiveBeginPlay`
  (`AudioComponent.SetSound` (`self.ticker`) "/Game/artSource/sounds/ticking_Cue.ticking_Cue")
  (bind _outactors (`GameplayStatics.GetAllActorsOfClass` "/Game/Blueprints/tools/toggleDoor.toggleDoor_C"))
  (for _array_element _outactors
    (if (`self.ActorHasTag` _array_element (`self.doorName`))
      (`KismetArrayLibrary.Array_Add` (`self.timedDoors`) _array_element))))

(event `self.Sphere.OnComponentHit`
  (params (OtherActor :type "Actor Object Reference") (OtherComp :type "PrimitiveComponent Object Reference") (NormalImpulse :type "Vector Structure") (Hit :type "HitResult Structure (by ref)"))
  (bind _astoggle_door (cast `/Game/Blueprints/tools/toggleDoor` (`self.door`)))
  (switch `/Game/Blueprints/tools/triggerType` (`self.triggerType`)
    (:`NewEnumerator0`
      (`/Game/Blueprints/tools/toggleDoor.trigger` _astoggle_door)
      (`GameplayStatics.PlaySoundAtLocation` "/Game/Character/assets/sounds/hit.hit" (`self.K2_GetActorLocation`)))
    (:`NewEnumerator1`
      (`SceneComponent.SetVisibility` (`self.TextRender`) true false)
      (`AudioComponent.Play` (`self.ticker`) 0.0)
      (for _array_element (`self.timedDoors`)
        (`/Game/Blueprints/tools/toggleDoor.trigger` _array_element))
      (bind _returnvalue (`KismetSystemLibrary.K2_SetTimer` null "openTimedDoors" (`self.openTime`)))
      (set `self.doorTimer` _returnvalue))))

(event `self.ReceiveActorBeginOverlap`
  (params (OtherActor :type "Actor Object Reference")))

(event `openTimedDoors`
  (for _array_element (`self.timedDoors`)
    (`/Game/Blueprints/tools/toggleDoor.trigger` _array_element)
    (`GameplayStatics.PlaySoundAtLocation` "/Game/Character/assets/sounds/beep.beep" (`self.K2_GetActorLocation` _array_element))
    (`AudioComponent.Stop` (`self.ticker`)))
  (`SceneComponent.SetVisibility` (`self.TextRender`) true false))

(event `self.ReceiveTick`
  (params (DeltaSeconds :type "Float (single-precision)"))
  (bind _textrender (`self.TextRender`))
  (bind _returnvalue (`KismetSystemLibrary.K2_GetTimerRemainingTimeHandle` (`self.doorTimer`)))
  (`SceneComponent.K2_SetRelativeRotation` _textrender (`KismetMathLibrary.FindLookAtRotation` (`self.K2_GetActorLocation`) (`self.K2_GetActorLocation` (`Controller.K2_GetPawn` (`GameplayStatics.GetPlayerController` 0)))) false false)
  (if (> _returnvalue 0.0)
    (`TextRenderComponent.K2_SetText` _textrender (`KismetTextLibrary.Conv_IntToText` (`KismetMathLibrary.FFloor` _returnvalue)))
    (else
      (`SceneComponent.SetVisibility` _textrender false false))))

(fn `UserConstructionScript`
  (bind _triggermesh (`self.triggerMesh`))
  (bind _sphere (`self.Sphere`))
  (`StaticMeshComponent.SetStaticMesh` _triggermesh (`self.triggerAppearance`))
  (`SceneComponent.K2_SetRelativeTransform` _triggermesh (`self.trigger Transform`) false false)
  (`SphereComponent.SetSphereRadius` _sphere (`self.collision Size`) true)
  (`SceneComponent.SetVisibility` _sphere (`self.show collision`) false)
  (bind _astoggle_door (cast `/Game/Blueprints/tools/toggleDoor` (`self.door`)))
  (bind _returnvalue (`PrimitiveComponent.CreateDynamicMaterialInstance` (`self.triggerMesh`) 0 "/Game/artSource/materials/doorIndicator_M.doorIndicator_M"))
  (bind _lockcolor (`/Game/Blueprints/tools/toggleDoor.lockColor` _astoggle_door))
  (`MaterialInstanceDynamic.SetVectorParameterValue` _returnvalue "color" _lockcolor)
  (`SceneComponent.K2_SetRelativeTransform` (`self.Sphere`) (`self.sphere transform`) false false)
  (`TextRenderComponent.SetTextRenderColor` (`self.TextRender`) (`KismetMathLibrary.Conv_LinearColorToColor` _lockcolor)))