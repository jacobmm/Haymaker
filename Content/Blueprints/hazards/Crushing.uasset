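; Crusher hazard that slams a moving volume toward a target actor and damages the player caught between them.
; A timeline lerps the volume to CrushingActor's location and a timer reverses it, cycling after a start delay if looping, otherwise triggered by the player entering a sphere.
; Damage requires a living player overlapping both, gated by a DoOnce that resets when the timeline finishes.
; The construction script applies configurable mesh, transforms, extent and radius.
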(event `self.ReceiveBeginPlay`
  (`TimelineComponent.SetPlayRate` (`self.moveCrushing`) (/ 1.0 (`self.speed in seconds`)))
  (set `self.start Location` (`SceneComponent.K2_GetComponentLocation` (`self.movingSmash`)))
  (set `self.crushingMeshWorldLoc` (`self.K2_GetActorLocation` (`self.crushingActor`)))
  (if (`self.crushing loop`)
    (`KismetSystemLibrary.Delay` (`self.startDelay`))
    (`self.moveDown`)
    (`KismetSystemLibrary.K2_SetTimer` null "moveDown" (* (/ (`self.speed in seconds`) 1.0) 2.0) true)))

(event `moveDown`
  (bind _movingsmash (`self.movingSmash`))
  (bind _crushingmeshworldloc (`self.crushingMeshWorldLoc`))
  (`KismetSystemLibrary.K2_SetTimer` null "reverse" (* (`self.speed in seconds`) 1.0) true)
  (set `self.direction` 0)
  (bind (_direction _alpha) (`Timeline|moveCrushing` :!label _label)
    (:`Update`
      (switch `int` (`self.direction`)
        (:`0`
          (`SceneComponent.K2_SetWorldLocation` _movingsmash (`KismetMathLibrary.VLerp` (`self.start Location`) _crushingmeshworldloc _alpha) false false))
        (:`1`
          (`SceneComponent.K2_SetWorldLocation` _movingsmash (`KismetMathLibrary.VLerp` (`self.start Location`) _crushingmeshworldloc _alpha) false false))))
    (:`Finished`
      (goto _label_2 :!via `Reset`))))

(event `reverse`
  (set `self.direction` 1)
  (goto _label :!via `Reverse`))

(event `self.ReceiveActorBeginOverlap`
  (params (OtherActor :type "Actor Object Reference")))

(event `self.Sphere.OnComponentBeginOverlap`
  (params (OtherActor :type "Actor Object Reference") (OtherComp :type "PrimitiveComponent Object Reference") (OtherBodyIndex :type Integer) (bFromSweep :type Boolean) (SweepResult :type "HitResult Structure (by ref)"))
  (bind _asmy_character (cast `/Game/Blueprints/MyCharacter` OtherActor))
  (set `self.player` OtherActor)
  (if (and (== OtherActor _asmy_character) (!= (`self.crushing loop`) true))
    (`self.moveDown`)))

(event `self.movingSmash.OnComponentBeginOverlap`
  (params (OtherActor :type "Actor Object Reference") (OtherComp :type "PrimitiveComponent Object Reference") (OtherBodyIndex :type Integer) (bFromSweep :type Boolean) (SweepResult :type "HitResult Structure (by ref)"))
  (bind _asmy_character (cast `/Game/Blueprints/MyCharacter` OtherActor))
  (if (== OtherActor _asmy_character)
    (if (and (`self.IsOverlappingActor` OtherActor (`self.crushingActor`)) (!= (`/Game/Blueprints/MyCharacter.dead` _asmy_character) true))
      (`/Engine/EditorBlueprintResources/StandardMacros.DoOnce` false :!label _label_2
        (:`Completed`
          (`GameplayStatics.ApplyDamage` OtherActor 150.0 null self "/Script/Engine.DamageType"))))))

(fn `UserConstructionScript`
  (bind _movingsmash (`self.movingSmash`))
  (`BoxComponent.SetBoxExtent` _movingsmash (`self.crushing volume extent`) true)
  (`SceneComponent.K2_SetRelativeTransform` _movingsmash (`self.crushingVolume Transform`) false false)
  (`SceneComponent.K2_SetRelativeTransform` (`self.StaticMesh`) (`self.crushingMesh Transform`) false false)
  (`StaticMeshComponent.SetStaticMesh` (`self.StaticMesh`) (`self.CrushingMesh`))
  (`SphereComponent.SetSphereRadius` (`self.Sphere`) (`self.radius`) true))