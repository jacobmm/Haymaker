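; Evil eye hazard that watches for the player character inside a configurable sphere and follows them with a beam.
; Shortly after the player enters, Tick eases the eye's rotation and a lagging beam target point toward them, both using one tracking strength.
; A visibility trace to that point spawns an impact emitter when it hits the player; no damage is applied here.
; Any end overlap stops tracking and resets the point.
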(event `self.ReceiveBeginPlay`
  (set `self.targetPoint` (`self.K2_GetActorLocation`)))

(event `self.ReceiveTick`
  (params (DeltaSeconds :type "Float (single-precision)"))
  (bind _targetpoint (`self.targetPoint`))
  (bind _staticmesh (`self.StaticMesh`))
  (bind _returnvalue (`SceneComponent.K2_GetComponentLocation` _staticmesh))
  (if (`self.targetLive`)
    (`SceneComponent.K2_SetRelativeRotation` _staticmesh (`KismetMathLibrary.RInterpTo` (`SceneComponent.RelativeRotation` _staticmesh) (`KismetMathLibrary.MakeRotator` (.roll (`KismetMathLibrary.FindLookAtRotation` _returnvalue (`self.K2_GetActorLocation` (`self.target`)))) (.pitch (`KismetMathLibrary.FindLookAtRotation` _returnvalue (`self.K2_GetActorLocation` (`self.target`)))) (+ (.yaw (`KismetMathLibrary.FindLookAtRotation` _returnvalue (`self.K2_GetActorLocation` (`self.target`)))) -90.0)) DeltaSeconds (`self.trackingSTrength`)) false false)
    (`self.trackPlayer`)
    (`self.beam` _targetpoint _returnvalue)
    (`ParticleSystemComponent.SetBeamTargetPoint` (`self.evilBeam`) 0 _targetpoint 0)
    (else
      (set `self.targetPoint` (`self.K2_GetActorLocation`)))))

(event `self.Sphere.OnComponentBeginOverlap`
  (params (OtherActor :type "Actor Object Reference") (OtherComp :type "PrimitiveComponent Object Reference") (OtherBodyIndex :type Integer) (bFromSweep :type Boolean) (SweepResult :type "HitResult Structure (by ref)"))
  (bind _asmy_character (cast `/Game/Blueprints/MyCharacter` OtherActor))
  (if (== _asmy_character OtherActor)
    (set `self.target` OtherActor)
    (`KismetSystemLibrary.Delay` 0.2)
    (set `self.targetLive` true)))

(event `self.Sphere.OnComponentEndOverlap`
  (params (OtherActor :type "Actor Object Reference") (OtherComp :type "PrimitiveComponent Object Reference") (OtherBodyIndex :type Integer))
  (set `self.targetLive` false))

(fn `beam`
  (params (targetLocation :type "Vector Structure") (myLocation :type "Vector Structure"))
  (bind _outhit (`KismetSystemLibrary.LineTraceSingle` :`Start` myLocation :`End` targetLocation :`TraceChannel` "TraceTypeQuery1" :`DrawDebugType` "ForOneFrame"))
  (bind (_bblockinghit _binitialoverlap _time _location _impactpoint _normal _impactnormal _physmat _hitactor) (`GameplayStatics.BreakHitResult` _outhit))
  (if (== _hitactor (`self.target`))
    (`GameplayStatics.SpawnEmitterAtLocation` "/Game/Blueprints/tools/checkDot.checkDot" _impactpoint)))

(fn `trackPlayer`
  (set `self.targetPoint` (`KismetMathLibrary.VInterpTo` (`self.targetPoint`) (`self.K2_GetActorLocation` (`self.target`)) (`GameplayStatics.GetWorldDeltaSeconds`) (`self.trackingSTrength`))))

(fn `UserConstructionScript`
  (`SphereComponent.SetSphereRadius` (`self.Sphere`) (`self.radius`) true)
  (`SceneComponent.K2_SetRelativeTransform` (`self.StaticMesh`) (`self.eyeTransform`) false false))