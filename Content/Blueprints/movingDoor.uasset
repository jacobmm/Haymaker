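; Configurable moving door that opens when MyCharacter enters its trigger, unless locked, and closes on exit unless set to one-time use.
; A timeline lerps the mesh's relative position and rotation, with play rate derived from travel time.
; Open and Close events drive the timeline directly, while CheckLocked clears the lock.
; The construction script sizes the trigger up from the ground, places the mesh and can preview the end pose.
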(event `self.doorTrigger.OnComponentBeginOverlap`
  (params (OtherActor :type "Actor Object Reference") (OtherComp :type "PrimitiveComponent Object Reference") (OtherBodyIndex :type Integer) (bFromSweep :type Boolean) (SweepResult :type "EngineTypes.HitResult Structure (by ref)"))
  ;[1 1 1] block moving control
  (bind _asmy_character (cast `/Game/Blueprints/MyCharacter` OtherActor))
  (if (== _asmy_character OtherActor)
    (if (`self.locked`)
      (`KismetSystemLibrary.PrintString` "Door Locked")
      (else
        (bind (_direction _lerp_position_alpha _lerp_rotation_alpha) (`Timeline|doorTimeline` :!via `PlayFromStart` :!label _label)
          (:`Update`
            (`SceneComponent.K2_SetRelativeLocationAndRotation` (`self.doorMesh`) (`KismetMathLibrary.VLerp` (`self.DoorLocation`) (`self.endPosition`) _lerp_position_alpha) (`KismetMathLibrary.RLerp` (struct) (`self.rotationScale`) _lerp_rotation_alpha) false))
          (:`Finished`
            (`KismetSystemLibrary.RetriggerableDelay` (`self.stopDelay`))
            ;;[1 1 1] us
            (switch `TimelineComponent.ETimelineDirection` _direction)))))))

(event `Open`
  ;[1 1 1] block moving control
  (goto _label :!via `PlayFromStart`))

(event `self.doorTrigger.OnComponentEndOverlap`
  (params (OtherActor :type "Actor Object Reference") (OtherComp :type "PrimitiveComponent Object Reference") (OtherBodyIndex :type Integer))
  ;[1 1 1] block moving control
  (bind _asmy_character (cast `/Game/Blueprints/MyCharacter` OtherActor))
  (if (== _asmy_character OtherActor)
    (if (not (`self.oneTimeUse`))
      (goto _label :!via `ReverseFromEnd`))))

(event `Close`
  ;[1 1 1] block moving control
  (goto _label :!via `ReverseFromEnd`))

(event `self.switchPress`
  ;[1 1 1] block moving control
  ;;[1 1 1] Trigger door on button press
)

(event `self.checkLocked`
  ;[1 1 1] block moving control
  (set `self.locked` false))

(event `self.ReceiveBeginPlay`
  (`TimelineComponent.SetPlayRate` (`self.doorTimeline`) (/ 1.0 (`self.travelTimeInSeconds`))))

(fn `UserConstructionScript`
  (bind _doormesh (`self.doorMesh`))
  (bind _doortrigger (`self.doorTrigger`))
  (bind _triggerscale (`self.TriggerScale`))
  ;[1 1 1] trigger size and location (Z scales up from the ground.)
  (`SceneComponent.SetRelativeScale3D` _doortrigger _triggerscale)
  (`SceneComponent.K2_SetRelativeLocation` _doortrigger (`KismetMathLibrary.MakeVector` (.x (`self.TriggerLocation`)) (.y (`self.TriggerLocation`)) (+ (.z (`self.TriggerLocation`)) (/ (* (.z _triggerscale) 60.0) 2.0))) false)
  ;[1 1 1] rotation
  (set `self.rotationScale` (`KismetMathLibrary.MakeRot` (`self.EndPitch`) (`self.EndYaw`) (`self.EndRoll`)))
  ;[1 1 1] Door location and scale
  (`SceneComponent.K2_SetRelativeLocation` _doormesh (`self.DoorLocation`) false)
  (`SceneComponent.SetRelativeScale3D` _doormesh (`self.DoorScale`))
  ;[1 1 1] test end position and rotation
  (`SceneComponent.K2_SetRelativeLocationAndRotation` (`self.doorMesh`) (`KismetMathLibrary.SelectVector` (`self.endPosition`) (`self.DoorLocation`) (`self.testEndPostion`)) (`KismetMathLibrary.SelectRotator` (`self.rotationScale`) (struct) (`self.TestEndRotation`)) false))