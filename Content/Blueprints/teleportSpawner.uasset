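; Spawner actor that builds a row of TeleportScreen actors at BeginPlay and reveals them one at a time.
; Each screen's SceneCapture hides the components of the next screen in the array, wrapping at the end.
; The screens are spaced evenly along negative Y, have their captures updated and start hidden.
; A replaying timeline acts as the timer, counting down through the array to unhide a screen each time it finishes.
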(event `self.ReceiveBeginPlay`
  (bind _telemesh (`self.teleMesh`))
  (for _ (range 51)
    (bind _returnvalue (`|SpawnActorFromClass` "/Game/artSource/Meshes/FX/teleportScreen.teleportScreen_C" (`KismetMathLibrary.MakeTransform` (`self.K2_GetActorLocation`) (struct) (`self.scale`)) "Undefined" "OverrideRootScale"))
    (`self.SetActorHiddenInGame` _returnvalue true)
    (`KismetArrayLibrary.Array_Add` _telemesh _returnvalue))
  (for (_array_element _array_index) _telemesh
    (`SceneCaptureComponent.HideActorComponents` (`/Game/artSource/Meshes/FX/teleportScreen.SceneCaptureComponent2D` _array_element) (`KismetArrayLibrary.Array_Get` _telemesh (mod (+ _array_index 1) (`KismetArrayLibrary.Array_Length` _telemesh)))))
  (set `self.location` (`self.K2_GetActorLocation`))
  (for _array_element_2 _telemesh
    (bind _output_get (set `self.location` (+ (`self.location`) (0.0 -80.0 0.0))))
    (`self.K2_SetActorLocation` _array_element_2 _output_get false false)
    (`/Game/artSource/Meshes/FX/teleportScreen.updateCaptureActor` _array_element_2)
    (`self.SetActorHiddenInGame` _array_element_2 true))
  (set `self.NewVar_0` (`KismetArrayLibrary.Array_Length` _telemesh))
  (`Timeline|Timeline_0` :!label _label
    (:`Finished`
      (bind _result (`/Engine/EditorBlueprintResources/StandardMacros.DecrementInt` (`self.NewVar_0`))
        (:`  `
          (`self.SetActorHiddenInGame` (`KismetArrayLibrary.Array_Get` _telemesh _result) false)
          (goto _label :!via `PlayFromStart`))))))

(event `self.ReceiveActorBeginOverlap`
  (params (OtherActor :type "Actor Object Reference")))

(event `self.ReceiveTick`
  (params (DeltaSeconds :type "Float (single-precision)")))

(fn `UserConstructionScript`)