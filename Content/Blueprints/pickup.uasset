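; Pickup actor that grants the player the device, spinning and bobbing on Tick via rotation and the PickupBob timeline.
; SwitchPress sets HasDevice on the controller's MyCharacter, unhides its gear, then hides the pickup mesh and disables its collision.
; It also records the gain in the haymaker GameInstance and, once only, opens the first ToggleDoor found in the level through OpenWithSwitch.
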(event `/Game/Blueprints/tools/buttonInteraction_BPI.switchPress`
  (params (myController :type "PlayerController Object Reference"))
  (bind _devicepickup (`self.devicePickup`))
  (bind _asmy_character (cast `/Game/Blueprints/MyCharacter` (`Controller.K2_GetPawn` myController)))
  (set `/Game/Blueprints/MyCharacter.hasDevice` true _asmy_character)
  (`/Game/Blueprints/MyCharacter.unhideGear` _asmy_character)
  (`SceneComponent.SetVisibility` _devicepickup false false)
  (`PrimitiveComponent.SetCollisionEnabled` _devicepickup "NoCollision")
  (bind _ashaymaker_gameinstance (cast `/Game/Blueprints/haymkaerBP/haymakerGameinstance` (`GameplayStatics.GetGameInstance`)))
  (`/Game/Blueprints/haymkaerBP/haymakerGameinstance.gainDevice` _ashaymaker_gameinstance)
  (`/Engine/EditorBlueprintResources/StandardMacros.DoOnce` false
    (:`Completed`
      (bind _outactors (`GameplayStatics.GetAllActorsOfClass` "/Game/Blueprints/tools/toggleDoor.toggleDoor_C"))
      (`/Game/Blueprints/tools/toggleDoor.openWithSwitch` (`KismetArrayLibrary.Array_Get` _outactors)))))

(event `self.ReceiveTick`
  (params (DeltaSeconds :type "Float (single-precision)"))
  (bind _devicepickup (`self.devicePickup`))
  (`SceneComponent.K2_AddLocalRotation` _devicepickup (struct :`Yaw` 0.6) false false)
  (bind (_direction _bob) (`Timeline|pickupBob`)
    (:`Update`
      (`SceneComponent.K2_AddLocalOffset` _devicepickup _bob false false))))

(fn `UserConstructionScript`)