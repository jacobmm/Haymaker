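; Configurable door block that slides or rotates when MyCharacter enters its trigger while unlocked, or when SwitchPress is called.
; The MovingBlock timeline adds a fixed local offset or rotation on every update, making travel frame-rate dependent.
; Unless OneTimeUse is set, leaving the trigger negates the offset (not rotation) and replays the timeline.
; CheckLocked clears the lock, and the construction script applies initial scale, location and rotation.
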(event `self.doorTrigger.OnComponentBeginOverlap`
  (params (OtherActor :type "Actor Object Reference") (OtherComp :type "PrimitiveComponent Object Reference") (OtherBodyIndex :type Integer) (bFromSweep :type Boolean) (SweepResult :type "EngineTypes.HitResult Structure (by ref)"))
  (bind _movingbock (`self.movingBock`))
  ;[1 1 1] block moving control
  (bind _asmy_character (cast `/Game/Blueprints/MyCharacter` OtherActor))
  (if (== _asmy_character OtherActor)
    (if (not (`self.locked`))
      (if (`self.oneTimeUse`)
        (`/Engine/EditorBlueprintResources/StandardMacros.DoOnce` false
          (:`Completed`
            _)))
      (set `self.moveDirection` (`KismetMathLibrary.MakeVector` (`self.X`) (`self.Y`) (`self.Z`)))
      (set `self.setRotation` (`KismetMathLibrary.MakeRot` (`self.pitch`) (`self.yaw`) (`self.roll`)))
      (`TimelineComponent.SetTimelineLength` (`self.timellineLenght`))
      (`Timeline|movingBlock` :!via `PlayFromStart` :!label _label
        (:`Update`
          (if (`self.rotator`)
            (`SceneComponent.K2_AddLocalRotation` _movingbock (`self.setRotation`) false)
            (else
              (`SceneComponent.K2_AddLocalOffset` _movingbock (`self.moveDirection`) false))))))))

(event `self.doorTrigger.OnComponentEndOverlap`
  (params (OtherActor :type "Actor Object Reference") (OtherComp :type "PrimitiveComponent Object Reference") (OtherBodyIndex :type Integer))
  ;[1 1 1] block moving control
  (bind _asmy_character (cast `/Game/Blueprints/MyCharacter` OtherActor))
  (if (== _asmy_character OtherActor)
    (if (not (`self.oneTimeUse`))
      (set `self.moveDirection` (* (`self.moveDirection`) -1.0))
      (goto _label :!via `PlayFromStart`))))

(event `self.switchPress`
  ;[1 1 1] block moving control
  ;;[1 1 1] Trigger door on button press
  (goto _label :!via `PlayFromStart`))

(event `self.checkLocked`
  ;[1 1 1] block moving control
  (set `self.locked` false))

(fn `UserConstructionScript`
  (bind _movingbock (`self.movingBock`))
  (`SceneComponent.SetRelativeScale3D` _movingbock (`KismetMathLibrary.MakeVector` (`self.xScale`) (`self.yScale`) (`self.zScale`)))
  (`SceneComponent.K2_SetRelativeLocationAndRotation` _movingbock (`self.initialLoc`) (`self.initialRot`) false))