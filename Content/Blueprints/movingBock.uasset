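; Configurable moving block that, after a start delay, either shuttles back and forth or spins continuously.
; A timeline of configurable length applies a fixed local offset or rotation on each update, selected by the Rotator flag, so speed depends on frame rate.
; When the timeline finishes, it negates the move direction and restarts; rotation keeps its direction.
; The construction script sets the block's scale from per-axis variables.
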(event `self.ReceiveBeginPlay`
  (bind _movingbock (`self.movingBock`))
  ;[1 1 1] block moving control
  (set `self.moveDirection` (`KismetMathLibrary.MakeVector` (`self.X`) (`self.Y`) (`self.Z`)))
  (set `self.setRotation` (`KismetMathLibrary.MakeRot` (`self.pitch`) (`self.yaw`) (`self.roll`)))
  (`KismetSystemLibrary.Delay` (`self.delayTime`))
  (`TimelineComponent.SetTimelineLength` (`self.timellineLenght`))
  (`Timeline|movingBlock` :!label _label
    (:`Update`
      (if (`self.rotator`)
        (`SceneComponent.K2_AddLocalRotation` _movingbock (`self.setRotation`) false)
        (else
          (`SceneComponent.K2_AddLocalOffset` _movingbock (`self.moveDirection`) false))))
    (:`Finished`
      (set `self.moveDirection` (* (`self.moveDirection`) -1.0))
      (goto _label :!via `PlayFromStart`))))

(fn `UserConstructionScript`
  (`SceneComponent.SetRelativeScale3D` (`self.movingBock`) (`KismetMathLibrary.MakeVector` (`self.xScale`) (`self.yScale`) (`self.zScale`))))