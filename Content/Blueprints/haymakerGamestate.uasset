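; Game state that times the player's level runs, keeps the fastest time per level and enforces an overall time budget.
; Runs count only after checkpoint B; finishing a level stores its best run and re-sums per-level bests into MyOTU.
; While in a level, Tick projects that total with the live time and, at OTM, clears runs and calls TakePlayerHome.
; Best times and total persist through a SaveSetup_BP save slot.
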(event EventLevelFinish
  (params (curLevel :type levelEnum%20Enum :default "NewEnumerator24"))
  ;[1 1 1] level Timers
  (CallFunction|StoreFastestTime curLevel)
  (CallFunction|ClearRuns)
  (CallFunction|CalcOTU))

(event EventGetAverageTime
  ;[1 1 1] level Timers
  (CallFunction|AverageTimes))

(event EventLoadGame
  (bind _returnvalue (SaveGame|LoadGamefromSlot "myGame"))
  (bind _assave_setup_bp (Utilities|Casting|CastToSaveSetup_BP _returnvalue))
  (Variables|Default|SetplayerFastestTimes (Variables|/Game/Blueprints/tools/SaveSetup_BP.SaveSetup_BP_C|GetsavedLevelTimes _assave_setup_bp))
  (bind _output_get (Variables|Default|SetmyOTU (Variables|/Game/Blueprints/tools/SaveSetup_BP.SaveSetup_BP_C|GetsavedOTU _assave_setup_bp)))
  (Development|PrintString (Utilities|String|ToString(Float) _output_get)))

(event EventSaveGame
  (bind _myotu (Variables|Default|GetmyOTU))
  (bind _returnvalue (SaveGame|CreateSaveGameObject "/Game/Blueprints/tools/SaveSetup_BP.SaveSetup_BP_C"))
  (bind _assave_setup_bp (Utilities|Casting|CastToSaveSetup_BP _returnvalue))
  (bind _output_get (Variables|Default|SetmySave _assave_setup_bp))
  (Variables|/Game/Blueprints/tools/SaveSetup_BP.SaveSetup_BP_C|SetsavedLevelTimes _output_get (Variables|Default|GetplayerFastestTimes))
  (Variables|/Game/Blueprints/tools/SaveSetup_BP.SaveSetup_BP_C|SetsavedOTU _output_get _myotu)
  (SaveGame|SaveGametoSlot (Variables|Default|GetmySave) "myGame")
  (Development|PrintString (Utilities|String|ToString(Float) _myotu)))

(event EventStartTimer
  ;[1 1 1] level Timers
  (Development|PrintString "Timer has begun.")
  (Variables|Default|SetStartTime (Math|DateTime|Now))
  (Variables|Default|SetinLevelNow true)
  (Variables|Default|SetpointB false))

(event EventEndTimer
  ;[1 1 1] level Timers
  (if (Variables|Default|GetpointB)
    (Development|PrintString "level has ended")
    (Variables|Default|SetElapsed%20Time (Math|DateTime|Now))
    (CallFunction|CalcTime)
    (CallFunction|AddTimes)
    (Variables|Default|SetinLevelNow false)
    (else
      (Development|PrintString "check point B not reached."))))

(event EventTick
  (params (DeltaSeconds :type Float%20%28single-precision%29))
  (if (Variables|Default|GetinLevelNow)
    (bind _bootme (CallFunction|StoreSecondsandTOTU))
    (if _bootme
      (CallFunction|ClearRuns)
      (bind _asmy_character (Utilities|Casting|CastToMyCharacter (Pawn|GetControlledPawn (Game|GetPlayerController 0))))
      (Default|TakePlayerHome _asmy_character))))

(event EventCheckPointB
  ;[1 1 1] level Timers
  (Variables|Default|SetpointB true))

(fn ConstructionScript)

(fn CalcTime
  (Variables|Default|SetcurrentRun (Math|Timespan|GetTotalSeconds (- (TimeOfDay|GetTimeOfDay (Variables|Default|GetElapsed%20Time) :!class /Script/Engine.KismetMathLibrary) (TimeOfDay|GetTimeOfDay (Variables|GetStartTime) :!class /Script/Engine.KismetMathLibrary)))))

(fn AverageTimes
  (bind _allruns (Variables|Default|GetAllRuns))
  (bind _allruns_2 (Variables|Default|GetAllRuns))
  (for (_ _array_index) _allruns
    (Development|PrintString (Utilities|String|ToString(Float) (Utilities|Array|Get(acopy) _allruns _array_index)) true true "(R=0.615700,G=0.802778,B=0.940000,A=1.000000)"))
  (Development|PrintString "Last 5 Run times")
  (Development|PrintString (Utilities|String|Append "Average Time: " (Utilities|String|ToString(Float) (/ (+ (Utilities|Array|Get(acopy) _allruns_2) (Utilities|Array|Get(acopy) _allruns_2 1) (Utilities|Array|Get(acopy) _allruns_2 2) (Utilities|Array|Get(acopy) _allruns_2 3) (Utilities|Array|Get(acopy) _allruns_2 4)) (Math|Conversions|ToFloat(Integer) (Utilities|Array|Length (Variables|Default|GetAllRuns)))))) true true "(R=0.283800,G=0.492165,B=0.645000,A=1.000000)")
  (Development|PrintString (Utilities|String|Append "Fastest Time: " (Utilities|String|ToString(Float) (.MinValue (Math|Float|MinOfFloatArray (Variables|Default|GetAllRuns))))) true true "(R=0.081650,G=0.239337,B=0.355000,A=1.000000)"))

(fn AddTimes
  (Utilities|Array|Add (Variables|Default|GetAllRuns) (Variables|Default|GetcurrentRun)))

(fn OverallTime)

(fn StoreFastestTime
  (params (selectedLevel :type levelEnum%20Enum))
  (bind _playerfastesttimes (Variables|Default|GetplayerFastestTimes))
  (bind _allruns (Variables|Default|GetAllRuns))
  (bind _minvalue (Math|Float|MinOfFloatArray _allruns))
  (bind _output_get (Variables|Default|SetselectedLevel selectedLevel))
  (bind _output_get_2 (LocalVariables|SetcurrentLevelByte (Math|Conversions|ToInteger(Byte) _output_get)))
  (Math|Float|CompareFloat _minvalue (Utilities|Array|Get(acopy) _playerfastesttimes _output_get_2) ; Make sure our "fastest time" is actually lower than our currently stored time.
    (:>
      (Math|Float|CompareFloat (Utilities|Array|Get(acopy) _playerfastesttimes _output_get_2) 0.0 ; If its 0, we haven't run this level yet, store the time.
        (:==
          _)))
    (:<
      _))
  (Utilities|Array|SetArrayElem _playerfastesttimes (LocalVariables|GetcurrentLevelByte) _minvalue)
  (return))

(fn ClearRuns
  (Utilities|Array|Clear (Variables|Default|GetAllRuns)))

(fn StoreSecondsandTOTU
  (bind _returnvalue (Math|DateTime|Now))
  (bind _starttime (Variables|Default|GetStartTime))
  (bind _returnvalue_2 (TimeOfDay|GetTimeOfDay _starttime :!class /Script/Engine.KismetMathLibrary))
  (bind _returnvalue_3 (TimeOfDay|GetTimeOfDay _returnvalue :!class /Script/Engine.KismetMathLibrary))
  (bind _returnvalue_4 (- _returnvalue_3 _returnvalue_2))
  (Variables|Default|SetmyCurrentTime _returnvalue_4)
  (bind _output_get (Variables|Default|SetmySeconds (Math|Timespan|GetTotalSeconds _returnvalue_4)))
  (bind _output_get_2 (Variables|Default|SetmyTempOTU (+ _output_get (- (Variables|Default|GetmyOTU) (Utilities|Array|Get(acopy) (Variables|Default|GetplayerFastestTimes) (Math|Conversions|ToInteger(Byte) (Variables|Default|GetselectedLevel)))))))
  (return (>= _output_get_2 (Variables|Default|GetOTM))))

(fn CalcOTU
  (for _array_element (Variables|Default|GetplayerFastestTimes)
    (LocalVariables|SetprevRunTime (+ _array_element (LocalVariables|GetprevRunTime))))
  (bind _output_get (Variables|Default|SetmyOTU (LocalVariables|GetprevRunTime)))
  (Development|PrintString (Utilities|String|ToString(Text) (Class|KismetTextLibrary|AsTimespanTimespan (Math|Timespan|FromSeconds _output_get))) true true "(R=0.160393,G=1.000000,B=0.000000,A=1.000000)"))