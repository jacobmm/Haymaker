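; Spline-based guide pipe actor that sends particle emitters along its length once the player character enters its spawn volume.
; The construction script builds the pipe from spline mesh segments between consecutive spline points.
; A self-rescheduling timer spawns particle components into an array.
; Tick advances them by a fixed per-frame step using a parallel distance array and destroys components that reach the spline's end.
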(event `spawnemitter`
  ;[1 1 1] emitter spawner
  (`KismetSystemLibrary.K2_SetTimer` null "spawnemitter" 2.0)
  (bind _returnvalue (`AddComponent|Particle System Component_184`))
  (`KismetArrayLibrary.Array_Add` (`self.particleArray`) _returnvalue))

(event `self.spawnVolume.OnComponentBeginOverlap`
  (params (OtherActor :type "Actor Object Reference") (OtherComp :type "PrimitiveComponent Object Reference") (OtherBodyIndex :type Integer) (bFromSweep :type Boolean) (SweepResult :type "HitResult Structure (by ref)"))
  ;[1 1 1] emitter spawner
  (bind _asmy_character (cast `/Game/Blueprints/MyCharacter` OtherActor))
  (if (== OtherActor _asmy_character)
    (`KismetSystemLibrary.K2_SetTimer` null "spawnemitter" 2.0)))

(event `self.ReceiveTick`
  (params (DeltaSeconds :type "Float (single-precision)"))
  (bind _particledistance (`self.particleDistance`))
  (for (_array_element _array_index) (`self.particleArray`)
    ;[1 1 1] destroy emitter and index
    (if (== (`SceneComponent.K2_GetComponentLocation` _array_element) (`SplineComponent.GetWorldLocationAtDistanceAlongSpline` (`self.Spline`) (`SplineComponent.GetSplineLength` (`self.Spline`))) :`ErrorTolerance` 0.0)
      (`ActorComponent.K2_DestroyComponent` _array_element)
      (`KismetSystemLibrary.PrintString` (`KismetSystemLibrary.GetDisplayName` _array_element))
      (`KismetArrayLibrary.Array_Remove` (`self.particleDistance`) _array_index)
      (else
        (set `self.particleInstPos` 0.0)
        (`KismetArrayLibrary.Array_Add` (`self.particleDistance`) (`self.particleInstPos`))
        (bind _item (`KismetArrayLibrary.Array_Get` _particledistance _array_index))
        (`KismetArrayLibrary.Array_Set` _particledistance _array_index (+ _item 55.0))
        (`SceneComponent.K2_SetWorldLocation` _array_element (`SplineComponent.GetWorldLocationAtDistanceAlongSpline` (`self.Spline`) _item) false)))))

(fn `UserConstructionScript`
  (bind _spline (`self.Spline`))
  (for _index (range (+ (- (`SplineComponent.GetNumSplinePoints` _spline) 2) 1))
    (bind _returnvalue (`AddComponent|Spline Mesh Component_0`))
    (`StaticMeshComponent.SetStaticMesh` _returnvalue (`self.NewVar`))
    (bind (_locallocation _localtangent) (`SplineComponent.GetLocalLocationAndTangentAtSplinePoint` _spline _index))
    (bind (_locallocation_2 _localtangent_2) (`SplineComponent.GetLocalLocationAndTangentAtSplinePoint` _spline (+ _index 1)))
    (`SplineMeshComponent.SetStartAndEnd` _returnvalue _locallocation _localtangent _locallocation_2 _localtangent_2)))