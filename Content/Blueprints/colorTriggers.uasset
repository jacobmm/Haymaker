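; A color trigger actor that changes its material color when hit by a MyProjectile.
; The construction script creates a dynamic material instance on the ColorTrigger component and stores it as DynamicTrigger.
; On a projectile hit, it sets that instance's baseColor parameter to Blue or Green, depending on the IsBlue flag, which this graph never changes.
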(event `self.ReceiveHit`
  (params (MyComp :type "PrimitiveComponent Object Reference") (Other :type "Actor Object Reference") (OtherComp :type "PrimitiveComponent Object Reference") (bSelfMoved :type Boolean) (HitLocation :type "Object.Vector Structure") (HitNormal :type "Object.Vector Structure") (NormalImpulse :type "Object.Vector Structure") (Hit :type "EngineTypes.HitResult Structure (by ref)"))
  (cast `/Game/Blueprints/MyProjectile` Other)
  (if (`self.isBlue`)
    (`MaterialInstanceDynamic.SetVectorParameterValue` (`self.dynamicTrigger`) "baseColor" (`KismetMathLibrary.Conv_VectorToLinearColor` (`self.blue`)))
    (else
      (`MaterialInstanceDynamic.SetVectorParameterValue` (`self.dynamicTrigger`) "baseColor" (`KismetMathLibrary.Conv_VectorToLinearColor` (`self.green`))))))

(fn `UserConstructionScript`
  (bind _returnvalue (`PrimitiveComponent.CreateDynamicMaterialInstance` (`self.colorTrigger`) 0 null))
  (set `self.dynamicTrigger` _returnvalue))