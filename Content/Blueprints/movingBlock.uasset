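; Moving block actor that shuttles between its origin and a configurable end position and rotation, after an initial start delay.
; A timeline, with play rate set by travel time, lerps the block's relative transform without sweep, then reverses after a stop delay at each end.
; The construction script applies scale, builds the end rotation, and uses test toggles to preview the end position and rotation.
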(event `self.ReceiveBeginPlay`
  ;[1 1 1] sets the speed of the moving block, rotation, and start delay
  (`TimelineComponent.SetPlayRate` (`self.movingBlockTimeline`) (/ 1.0 (`self.travelTimeInSeconds`)))
  (`KismetSystemLibrary.Delay` (`self.startDelay`))
  ;[1 1 1] block moving control
  (bind (_direction _lerp_position_alpha _lerp_rotation_alpha) (`Timeline|movingBlockTimeline` :!label _label)
    (:`Update`
      (`SceneComponent.K2_SetRelativeLocationAndRotation` (`self.movingBlock`) (`KismetMathLibrary.VLerp` (0.0 0.0 0.0) (`self.endPosition`) _lerp_position_alpha) (`KismetMathLibrary.RLerp` (struct) (`self.rotationScale`) _lerp_rotation_alpha) false))
    (:`Finished`
      (`KismetSystemLibrary.RetriggerableDelay` (`self.stopDelay`))
      (switch `TimelineComponent.ETimelineDirection` _direction
        (:`Forward`
          (`self.moveBackward`))
        (:`Backward`
          (`self.moveForward`))))))

(event `moveForward`
  ;[1 1 1] block moving control
  (goto _label :!via `PlayFromStart`))

(event `moveBackward`
  ;[1 1 1] block moving control
  (goto _label :!via `ReverseFromEnd`))

(fn `UserConstructionScript`
  ;[1 1 1] rotation
  (set `self.rotationScale` (`KismetMathLibrary.MakeRot` (`self.EndPitch`) (`self.EndYaw`) (`self.EndRoll`)))
  ;[1 1 1] set start delay
  (set `self.startDelay` (`self.startDelay`))
  ;[1 1 1] block scale
  (`SceneComponent.SetRelativeScale3D` (`self.movingBlock`) (`self.scale`))
  ;[1 1 1] test end position and rotation
  (`SceneComponent.K2_SetRelativeLocationAndRotation` (`self.movingBlock`) (`KismetMathLibrary.SelectVector` (`self.endPosition`) (0.0 0.0 0.0) (`self.testEndPostion`)) (`KismetMathLibrary.SelectRotator` (`self.rotationScale`) (struct) (`self.TestEndRotation`)) false))