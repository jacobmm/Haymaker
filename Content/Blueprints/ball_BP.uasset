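; Ball actor Blueprint that tints its mesh to match the ball color selected on the player's character.
; On BeginPlay it casts the first player's controlled pawn to MyCharacter and creates a dynamic instance of Ball_Inst on the static mesh.
; A switch on the character's MyBallColor sets the ballColor vector parameter to blue, green, white or red.
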(event `self.ReceiveBeginPlay`
  (bind _asmy_character (cast `/Game/Blueprints/MyCharacter` (`Controller.K2_GetPawn` (`GameplayStatics.GetPlayerController` 0))))
  (bind _returnvalue (`PrimitiveComponent.CreateDynamicMaterialInstance` (`self.StaticMesh`) 0 "/Game/artSource/materials/ball_Inst.ball_Inst"))
  (bind _output_get (set `self.NewVar` _returnvalue))
  (switch `/Game/Blueprints/tools/ballColor` (`/Game/Blueprints/MyCharacter.myBallColor` _asmy_character)
    (:`NewEnumerator0`
      (`MaterialInstanceDynamic.SetVectorParameterValue` _output_get "ballColor" (struct :`B` 1.0 :`A` 1.0)))
    (:`NewEnumerator1`
      (`MaterialInstanceDynamic.SetVectorParameterValue` _output_get "ballColor" (struct :`G` 1.0 :`A` 1.0)))
    (:`NewEnumerator2`
      (`MaterialInstanceDynamic.SetVectorParameterValue` _output_get "ballColor" (struct :`R` 1.0 :`G` 1.0 :`B` 1.0 :`A` 1.0)))
    (:`NewEnumerator3`
      (`MaterialInstanceDynamic.SetVectorParameterValue` _output_get "ballColor" (struct :`R` 1.0 :`A` 1.0)))))

(event `self.ReceiveActorBeginOverlap`
  (params (OtherActor :type "Actor Object Reference")))

(event `self.ReceiveTick`
  (params (DeltaSeconds :type "Float (single-precision)")))

(fn `UserConstructionScript`)