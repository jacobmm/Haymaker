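; Player controller for Haymaker that owns a travel menu for hosting games, joining games and changing levels.
; After a short delay on BeginPlay, the authority calls a client-named event that creates the menu widget hidden.
; An input action or toggle event switches its visibility and input mode, and EndPlay removes it.
; Server-named host, join and travel events forward to the haymakerGameinstance, which handles the session and travel work.
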(event `self.ReceiveBeginPlay`
  ;[1 1 1] create the menu on the client
  (`KismetSystemLibrary.Delay` 0.2)
  (`/Engine/EditorBlueprintResources/ActorMacros.Switch Has Authority`
    (:`Authority`
      (`self.clientTravelmenu`))))

(event `clientTravelmenu`
  ;[1 1 1] create the menu on the client
  (bind _returnvalue (`|CreateWidget` "/Game/Blueprints/umg/travelMenu.travelMenu_C" self))
  (bind _output_get (set `self.player_TravelMenu` _returnvalue))
  (`UserWidget.AddToViewport` _output_get 0)
  (`Widget.SetVisibility` _output_get "Hidden"))

(event `InputAction|Open Server Menu`
  (params (Key :type "Key Structure" :default "AnyKey"))
  (bind _player_travelmenu (`self.player_TravelMenu`))
  ;[1 1 1] hide and show menu
  (:`Pressed`
    (if (`|EnumEquality` (`Widget.GetVisibility` _player_travelmenu) "Visible") :!label _label
      (`Widget.SetVisibility` _player_travelmenu "Hidden")
      (`WidgetBlueprintLibrary.SetInputMode_GameOnly` self)
      (else
        (`Widget.SetVisibility` _player_travelmenu "Visible")
        (`WidgetBlueprintLibrary.SetInputMode_GameAndUIEx` self _player_travelmenu true false)))))

(event `toggleMenuPress`
  ;[1 1 1] hide and show menu
  (goto _label))

(event `serverHostGame`
  ;[1 1 1] Create new game
  (bind _ashaymaker_gameinstance (cast `/Game/Blueprints/haymkaerBP/haymakerGameinstance` (`GameplayStatics.GetGameInstance`)))
  (`/Game/Blueprints/haymkaerBP/haymakerGameinstance.serverHostGameInstance` _ashaymaker_gameinstance self))

(event `self.ReceiveEndPlay`
  (params (EndPlayReason :type "EEndPlayReason Enum" :default "Destroyed"))
  (bind _player_travelmenu (`self.player_TravelMenu`))
  ;[1 1 1] Create new game
  (`/Engine/EditorBlueprintResources/StandardMacros.IsValid` _player_travelmenu
    (:`Is Valid`
      (`Widget.RemoveFromParent` _player_travelmenu)
      (`WidgetBlueprintLibrary.SetInputMode_GameOnly` self))))

(event `serverJoinGame`
  ;[1 1 1] join game
  (bind _ashaymaker_gameinstance (cast `/Game/Blueprints/haymkaerBP/haymakerGameinstance` (`GameplayStatics.GetGameInstance`)))
  (`/Game/Blueprints/haymkaerBP/haymakerGameinstance.serverJoinGameInstance` _ashaymaker_gameinstance self))

(event `serverTravelToLevel`
  (params (levelName :type String))
  (bind _ashaymaker_gameinstance (cast `/Game/Blueprints/haymkaerBP/haymakerGameinstance` (`GameplayStatics.GetGameInstance`)))
  (`/Game/Blueprints/haymkaerBP/haymakerGameinstance.serverTravelToLevelInstance` _ashaymaker_gameinstance levelName))

(fn `UserConstructionScript`)