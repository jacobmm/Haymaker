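; Haymaker game instance that holds speedrun records and level progression, handles new and loaded games, and runs LAN multiplayer sessions.
; StoreTime keeps each level's best time, re-sums them into MyOTU, saves, then clears runs and updates level details to unlock the next level.
; Only best times and the OTU total persist, through SaveSetup_BP in one slot.
; Session events host a listen-server lobby, join the first found session, and servertravel between levels.
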(event Custom|trackStats
  (params (levelAttemps :type Integer) (Deaths :type Integer) (levelUnlock :type Integer))
  ;[1 1 1] score tracking
  (Variables|Default|SetlevelAttempts levelAttemps))

(event Custom|createLevelInfo
  (CallFunction|LevelInfoMaintence))

(event Custom|serverJoinGameInstance
  (params (Client :type Player%20Controller%20Object%20Reference))
  ;[1 1 1] join session
  (bind _results (|FindSessions Client 1 true)
    (:OnSuccess
      (|JoinSession Client (Utilities|Array|Get(acopy) _results)))
    (:OnFailure
      (Development|PrintString "failed to find session" true true "(R=1.000000,G=0.019354,B=0.000000,A=1.000000)"))))

(event Custom|newGame
  ;[1 1 1] start new game/load game
  (Game|OpenLevel(byName) "tut01" false))

(event Custom|loadOldGame
  ;[1 1 1] start new game/load game
  (CallFunction|LoadGame)
  (Game|OpenLevel(byName) "mainRoom"))

(event Custom|ClearTimer
  (Variables|Default|SetpointB false))

(event Custom|serverTravelToLevelInstance
  (params (level%20for%20travel :type String))
  (Development|ExecuteConsoleCommand (Utilities|String|Append "servertravel " level%20for%20travel) (Game|GetPlayerController 0)))

(event Custom|StoreTime
  (params (currentLevel :type levelEnum%20Enum) (FastestTime :type Float%20%28single-precision%29) (deaths :type Integer))
  (bind _returnvalue (Math|Conversions|ToInteger(Byte) currentLevel))
  ;[1 1 1] constantly check time
  (CallFunction|StoreFastestTime currentLevel FastestTime)
  (CallFunction|CalcOTU)
  (CallFunction|SaveGame)
  (bind _ashaymaker_gamestate (Utilities|Casting|CastTohaymakerGamestate (Game|GetGameState)))
  (Default|ClearRuns _ashaymaker_gamestate)
  (if (> FastestTime 0.0)
    (CallFunction|LevelDetailEditor _returnvalue (Utilities|Array|Get(acopy) (Variables|Default|GetplayerFastestTimes) _returnvalue) true deaths)
    (CallFunction|LevelDetailEditor (+ _returnvalue 1) 0.0 true)))

(event Custom|serverHostGameInstance
  (params (hostController :type Player%20Controller%20Object%20Reference))
  ;[1 1 1] create lobby level
  (|Session hostController 4 true
    (:OnSuccess
      (Game|OpenLevel(byName) "lobby" true "listen"))
    (:OnFailure
      (Development|PrintString "session not created" true true "(R=1.000000,G=0.000000,B=0.109699,A=1.000000)"))))

(event EventSaveGame
  ;[1 1 1] save and load game functions
  (bind _returnvalue (SaveGame|CreateSaveGameObject "/Game/Blueprints/tools/SaveSetup_BP.SaveSetup_BP_C"))
  (bind _assave_setup_bp (Utilities|Casting|CastToSaveSetup_BP _returnvalue))
  (bind _output_get (Variables|Default|SetmySave _assave_setup_bp))
  (Variables|/Game/Blueprints/tools/SaveSetup_BP.SaveSetup_BP_C|SetsavedLevelTimes _output_get (Variables|Default|GetplayerFastestTimes))
  (Variables|/Game/Blueprints/tools/SaveSetup_BP.SaveSetup_BP_C|SetsavedOTU _output_get (Variables|Default|GetmyOTU))
  (bind _returnvalue_2 (SaveGame|SaveGametoSlot (Variables|Default|GetmySave) "myGame"))
  (if (and _returnvalue_2 (Variables|Default|GetquitGame))
    (Game|QuitGame (Game|GetPlayerController 0) "Quit")))

(event EventLoadGame
  ;[1 1 1] save and load game functions
  (bind _returnvalue (SaveGame|LoadGamefromSlot "myGame"))
  (bind _assave_setup_bp (Utilities|Casting|CastToSaveSetup_BP _returnvalue))
  (Variables|Default|SetplayerFastestTimes (Variables|/Game/Blueprints/tools/SaveSetup_BP.SaveSetup_BP_C|GetsavedLevelTimes _assave_setup_bp))
  (Variables|Default|SetmyOTU (Variables|/Game/Blueprints/tools/SaveSetup_BP.SaveSetup_BP_C|GetsavedOTU _assave_setup_bp)))

(fn CalcTime
  (Variables|Default|SetcurrentRun (Math|Timespan|GetTotalSeconds (- (TimeOfDay|GetTimeOfDay (Variables|Default|GetElapsed%20Time) :!class /Script/Engine.KismetMathLibrary) (TimeOfDay|GetTimeOfDay (Variables|GetStartTime) :!class /Script/Engine.KismetMathLibrary)))))

(fn AverageTimes
  (bind _allruns (Variables|Default|GetAllRuns))
  (for (_ _array_index) _allruns
    (Development|PrintString (Utilities|String|ToString(Float) (Utilities|Array|Get(acopy) _allruns _array_index)) true true "(R=0.940000,G=0.940000,B=0.940000,A=1.000000)"))
  (Development|PrintString (Utilities|String|Append "Fastest Time: " (Utilities|String|ToString(Float) (.MinValue (Math|Float|MinOfFloatArray (Variables|Default|GetAllRuns))))) true true "(R=0.355000,G=0.000000,B=0.000000,A=1.000000)"))

(fn AddTimes
  (Utilities|Array|Add (Variables|Default|GetAllRuns) (Variables|Default|GetcurrentRun)))

(fn StoreFastestTime
  (params (selectedLevel :type levelEnum%20Enum) (NewParam :type Float%20%28single-precision%29))
  (bind _returnvalue (Math|Conversions|ToInteger(Byte) selectedLevel))
  (bind _playerfastesttimes (Variables|Default|GetplayerFastestTimes))
  (bind _item (Utilities|Array|Get(acopy) _playerfastesttimes _returnvalue))
  (Math|Float|CompareFloat _item 0.0
    (:>
      (Math|Float|CompareFloat NewParam _item
        (:<
          _)))
    (:==
      _))
  (Utilities|Array|SetArrayElem _playerfastesttimes _returnvalue NewParam))

(fn ClearRuns
  (Utilities|Array|Clear (Variables|Default|GetAllRuns)))

(fn StoreSecondsandTOTU
  (bind _returnvalue (Math|DateTime|Now))
  (bind _starttime (Variables|Default|GetStartTime))
  (bind _returnvalue_2 (TimeOfDay|GetTimeOfDay _starttime :!class /Script/Engine.KismetMathLibrary))
  (bind _returnvalue_3 (TimeOfDay|GetTimeOfDay _returnvalue :!class /Script/Engine.KismetMathLibrary))
  (bind _returnvalue_4 (- _returnvalue_3 _returnvalue_2))
  (Variables|Default|SetmyCurrentTime _returnvalue_4)
  (bind _output_get (Variables|Default|SetmySeconds (Math|Timespan|GetTotalSeconds _returnvalue_4)))
  (bind _output_get_2 (Variables|Default|SetmyTempOTU (+ _output_get (- (Variables|Default|GetmyOTU) (Utilities|Array|Get(acopy) (Variables|Default|GetplayerFastestTimes) (Math|Conversions|ToInteger(Byte) (Variables|Default|GetselectedLevel)))))))
  (return (>= _output_get_2 (Variables|Default|GetOTM))))

(fn CalcOTU
  (for _array_element (Variables|Default|GetplayerFastestTimes)
    (LocalVariables|SetprevRunTime (+ _array_element (LocalVariables|GetprevRunTime))))
  (bind _output_get (Variables|Default|SetmyOTU (LocalVariables|GetprevRunTime)))
  (Development|PrintString (Utilities|String|ToString(Text) (Class|KismetTextLibrary|AsTimespanTimespan (Math|Timespan|FromSeconds _output_get))) true true "(R=0.160393,G=1.000000,B=0.000000,A=1.000000)"))

(fn OnRepMyCurrentTime)

(fn LevelDetailEditor
  (params (levelToEdit :type Integer) (FastestTime :type Float%20%28single-precision%29) (levelCompleted :type Boolean) (deaths :type Integer))
  (Utilities|Struct|SetmembersinlevelDetail (Utilities|Array|Get(acopy) (Variables|Default|GetlevelDetailArray) levelToEdit) levelCompleted FastestTime deaths))

(fn LevelInfoMaintence
  (Variables|Default|SetlevelDetailArray (Utilities|Array|MakeArray (Variables|Default|Gettut01) (Variables|Default|Gettut02) (Variables|Default|Gettut03) (Variables|Default|Gettut04) (Variables|Default|Gettut05) (Variables|Default|Gettut06) (Variables|Default|Gettut07) (Variables|Default|Getlevel1) (Variables|Default|Getlevel2) (Variables|Default|Getlevel3) (Variables|Default|Getlevel4) (Variables|Default|Getlevel5) (Variables|Default|Getlevel6) (Variables|Default|Getlevel7) (Variables|Default|Getlevel8))))