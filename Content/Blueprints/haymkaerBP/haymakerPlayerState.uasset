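; Player state for the haymaker game that times a player's run.
; setStartTime stores the runner's controller and start timestamp and starts the timer; setEndTime stops it and records the end timestamp.
; While the timer runs, Tick computes elapsed time and total seconds by subtracting time-of-day values, so the date is ignored.
; The OnRep handler for the current time is empty.
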(event `self.ReceiveTick`
  (params (DeltaSeconds :type "Float (single-precision)"))
  (if (`self.startCurrentTime`)
    (bind _output_get (set `self.playerCurrentTime` (- (`KismetMathLibrary.GetTimeOfDay` (`KismetMathLibrary.Now`)) (`KismetMathLibrary.GetTimeOfDay` (`self.playerStartTime`)))))
    (set `self.playerSeconds` (`KismetMathLibrary.GetTotalSeconds` _output_get))))

(event `self.ReceiveBeginPlay`)

(event `setStartTime`
  (params (runner :type "PlayerController Object Reference"))
  (set `self.startCurrentTime` true)
  (set `self.runnerController` runner)
  (set `self.playerStartTime` (`KismetMathLibrary.Now`)))

(event `setEndTime`
  (set `self.startCurrentTime` false)
  (set `self.playerEndTime` (`KismetMathLibrary.Now`)))

(fn `OnRep_playerCurrentTime`)

(fn `UserConstructionScript`)