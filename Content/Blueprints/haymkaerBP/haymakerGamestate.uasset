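; Haymaker game state that times level runs and enforces an overall time limit.
; EndTimer records a run only after checkpoint B, otherwise restarting the timer; LevelFinish saves the fastest run to the game instance.
; While a run is active, Tick projects the overall total using stored level bests, clearing runs and sending the player home at the limit.
; Separate server events delegate multiplayer start and end times to each runner's PlayerState.
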(event Custom|serverLevelFinish
  (params (runner :type Player%20Controller%20Object%20Reference) (currentLevel :type levelEnum%20Enum))
  ;[1 1 1] level Timers
  (bind _ashaymaker_gameinstance (Utilities|Casting|CastTohaymakerGameinstance (Game|GetGameInstance)))
  (Default|StoreTime _ashaymaker_gameinstance (stale EventLevelFinish curLevel) (.MinValue (Math|Float|MinOfFloatArray (Variables|Default|GetAllRuns)))))

(event Custom|serverStartTimer
  (params (runner :type Player%20Controller%20Object%20Reference))
  ;[1 1 1] multiplayer timer
  (bind _ashaymaker_player_state (Utilities|Casting|CastTohaymakerPlayerState (Variables|/Script/Engine.Controller|GetPlayerState runner)))
  (Default|SetStartTime _ashaymaker_player_state runner))

(event Custom|serverEndTimer
  (params (runner :type Player%20Controller%20Object%20Reference))
  ;[1 1 1] multiplayer timer
  (bind _ashaymaker_player_state (Utilities|Casting|CastTohaymakerPlayerState (Variables|/Script/Engine.Controller|GetPlayerState runner)))
  (Default|SetEndTime _ashaymaker_player_state))

(event EventLevelFinish
  (params (curLevel :type levelEnum%20Enum :default "NewEnumerator24"))
  ;[1 1 1] level Timers
  (bind _ashaymaker_gameinstance (Utilities|Casting|CastTohaymakerGameinstance (Game|GetGameInstance)))
  (Default|StoreTime _ashaymaker_gameinstance curLevel (.MinValue (Math|Float|MinOfFloatArray (Variables|Default|GetAllRuns)))))

(event EventStartTimer
  ;[1 1 1] level Timers
  (Development|PrintString "Timer has begun.")
  (CallFunction|TrackTime))

(event EventEndTimer
  ;[1 1 1] level Timers
  (if (Variables|Default|GetpointB)
    (Development|PrintString "level has ended")
    (CallFunction|CalcTime)
    (CallFunction|AddTimes)
    (Variables|Default|SetinLevelNow false)
    (Variables|Default|SetpointB false)
    (else
      (Development|PrintString "check point B not reached.")
      (CallFunction|StartTimer))))

(event EventTick
  (params (DeltaSeconds :type Float%20%28single-precision%29))
  (if (Variables|Default|GetinLevelNow)
    (bind _bootme (CallFunction|StoreSecondsandTOTU))
    (if _bootme
      (CallFunction|ClearRuns)
      (bind _asmy_character (Utilities|Casting|CastToMyCharacter (Pawn|GetControlledPawn (Game|GetPlayerController 0))))
      (Default|TakePlayerHome _asmy_character))))

(event EventBeginPlay
  (bind _asmy_character (Utilities|Casting|CastToMyCharacter (Pawn|GetControlledPawn (Game|GetPlayerController 0))))
  (Variables|Default|SetselectedLevel (Variables|/Game/Blueprints/MyCharacter.MyCharacter_C|GetcurrentLevel _asmy_character)))

(event EventCheckPointB
  ;[1 1 1] level Timers
  (Variables|Default|SetpointB true))

(fn ConstructionScript)

(fn CalcTime
  (bind _output_get (Variables|Default|SetElapsed%20Time (Math|DateTime|Now)))
  (Variables|Default|SetcurrentRun (Math|Timespan|GetTotalSeconds (- (TimeOfDay|GetTimeOfDay _output_get :!class /Script/Engine.KismetMathLibrary) (TimeOfDay|GetTimeOfDay (Variables|GetStartTime) :!class /Script/Engine.KismetMathLibrary)))))

(fn AverageTimes
  (bind _allruns (Variables|Default|GetAllRuns))
  (bind _allruns_2 (Variables|Default|GetAllRuns))
  (for (_ _array_index) _allruns
    (Development|PrintString (Utilities|String|ToString(Float) (Utilities|Array|Get(acopy) _allruns _array_index)) true true "(R=0.615700,G=0.802778,B=0.940000,A=1.000000)"))
  (Development|PrintString "Last 5 Run times")
  (Development|PrintString (Utilities|String|Append "Average Time: " (Utilities|String|ToString(Float) (/ (+ (Utilities|Array|Get(acopy) _allruns_2) (Utilities|Array|Get(acopy) _allruns_2 1) (Utilities|Array|Get(acopy) _allruns_2 2) (Utilities|Array|Get(acopy) _allruns_2 3) (Utilities|Array|Get(acopy) _allruns_2 4)) (Math|Conversions|ToFloat(Integer) (Utilities|Array|Length (Variables|Default|GetAllRuns)))))) true true "(R=0.283800,G=0.492165,B=0.645000,A=1.000000)")
  (Development|PrintString (Utilities|String|Append "Fastest Time: " (Utilities|String|ToString(Float) (.MinValue (Math|Float|MinOfFloatArray (Variables|Default|GetAllRuns))))) true true "(R=0.081650,G=0.239337,B=0.355000,A=1.000000)"))

(fn AddTimes
  (Utilities|Array|Add (Variables|Default|GetAllRuns) (Variables|Default|GetcurrentRun)))

(fn OverallTime)

(fn CheckFastestTime
  (params (selectedLevel :type levelEnum%20Enum))
  (return 0.0))

(fn ClearRuns
  (Utilities|Array|Clear (Variables|Default|GetAllRuns)))

(fn StoreSecondsandTOTU
  (bind _returnvalue (Math|DateTime|Now))
  (bind _starttime (Variables|Default|GetStartTime))
  (bind _returnvalue_2 (TimeOfDay|GetTimeOfDay _starttime :!class /Script/Engine.KismetMathLibrary))
  (bind _returnvalue_3 (TimeOfDay|GetTimeOfDay _returnvalue :!class /Script/Engine.KismetMathLibrary))
  (bind _returnvalue_4 (- _returnvalue_3 _returnvalue_2))
  (bind _ashaymaker_gameinstance (Utilities|Casting|CastTohaymakerGameinstance (Game|GetGameInstance)))
  (Variables|Default|SetmyCurrentTime _returnvalue_4)
  (bind _output_get (Variables|Default|SetmySeconds (Math|Timespan|GetTotalSeconds _returnvalue_4)))
  (bind _output_get_2 (Variables|Default|SetmyTempOTU (+ _output_get (- (Variables|/Game/Blueprints/haymkaerBP/haymakerGameinstance.haymakerGameinstance_C|GetmyOTU _ashaymaker_gameinstance) (Utilities|Array|Get(acopy) (Variables|/Game/Blueprints/haymkaerBP/haymakerGameinstance.haymakerGameinstance_C|GetplayerFastestTimes _ashaymaker_gameinstance) (Math|Conversions|ToInteger(Byte) (Variables|Default|GetselectedLevel)))))))
  (return (>= _output_get_2 (Variables|/Game/Blueprints/haymkaerBP/haymakerGameinstance.haymakerGameinstance_C|GetOTM _ashaymaker_gameinstance))))

(fn TrackTime
  (Variables|Default|SetStartTime (Math|DateTime|Now))
  (Variables|Default|SetinLevelNow true))

(fn OnRepStartTime)

(fn OnRepElapsedTime)

(fn OnRepMySeconds)

(fn OnRepMyOTU)

(fn OnRepMyTempOTU)

(fn OnRepMyCurrentTime)