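; Game mode for haymaker that sets up level info and handles streaming level swaps.
; On BeginPlay it has the haymaker game instance create its level info.
; The loadLevel event reads the current level stored on the player character, unloads it unless it is the main room, then streams in the requested level.
; Level enum values convert directly to streaming level names, with debug prints reporting each step.
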(event `self.ReceiveBeginPlay`
  (bind _ashaymaker_gameinstance (cast `/Game/Blueprints/haymkaerBP/haymakerGameinstance` (`GameplayStatics.GetGameInstance`)))
  (`/Game/Blueprints/haymkaerBP/haymakerGameinstance.createLevelInfo` _ashaymaker_gameinstance))

(event `loadLevel`
  (params (levelToLoad :type "/Game/Blueprints/haymkaerBP/levelEnum Enum"))
  (bind _returnvalue (`|GetEnumeratorNameAsString` levelToLoad))
  ;[1 1 1] if in the mainRoom, load our new level. Otherwise unload the level that was stored on the player and load the new one.
  (bind _asmy_character (cast `/Game/Blueprints/MyCharacter` (`Controller.K2_GetPawn` (`GameplayStatics.GetPlayerController` 0))))
  (bind _currentlevel (`/Game/Blueprints/MyCharacter.currentLevel` _asmy_character))
  (if (`|EnumEquality` _currentlevel "NewEnumerator24")
    (if (not (`|EnumEquality` levelToLoad _currentlevel))
      (`GameplayStatics.LoadStreamLevel` (`KismetStringLibrary.Conv_StringToName` _returnvalue) true :!label _label)
      (`KismetSystemLibrary.PrintString` (`KismetStringLibrary.Concat_StrStr` "Finished loading " _returnvalue) true true (struct :`G` 1.0 :`B` 0.099808 :`A` 1.0)))
    (else
      (`GameplayStatics.UnloadStreamLevel` (`KismetStringLibrary.Conv_StringToName` (`|GetEnumeratorNameAsString` _currentlevel)))
      (`KismetSystemLibrary.PrintString` (`KismetStringLibrary.Concat_StrStr` "Just unloaded " (`|GetEnumeratorNameAsString` _currentlevel)) true true (struct :`R` 1.0 :`G` 0.648792 :`A` 1.0))
      (goto _label))))

(fn `UserConstructionScript`)