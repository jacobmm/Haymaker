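; Energy ring actor that recolors MyProjectile balls passing through it to red, green or blue.
; The construction script scales the ring and tints a dynamic material instance from its color booleans.
; When a projectile ends overlap, it switches that projectile's collision object channel and ball material color to match.
; It also sets the firing MyCharacter's ball color enum and calls DummyBallColor on it.
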(event `self.ReceiveActorEndOverlap`
  (params (OtherActor :type "Actor Object Reference"))
  (bind _returnvalue (`self.GetInstigator` OtherActor))
  (bind _asmy_projectile (cast `/Game/Blueprints/MyProjectile` OtherActor))
  (bind _asmy_character (cast `/Game/Blueprints/MyCharacter` _returnvalue))
  (if (`self.isRed`)
    (bind _collisioncomponent (`/Game/Blueprints/MyProjectile.CollisionComponent` _asmy_projectile))
    (`PrimitiveComponent.SetCollisionObjectType` _collisioncomponent "ECC_GameTraceChannel4")
    (bind _setballcolor (`/Game/Blueprints/MyProjectile.setBallColor` _asmy_projectile))
    (`MaterialInstanceDynamic.SetVectorParameterValue` _setballcolor "ballColor" (`self.redColor`))
    (bind _asmy_character_2 (cast `/Game/Blueprints/MyCharacter` _returnvalue))
    (set `/Game/Blueprints/MyCharacter.myBallColor` "NewEnumerator3" _asmy_character_2)
    (`/Game/Blueprints/MyCharacter.dummyBallColor` _asmy_character :!label _label)
    (elif (`self.isGreen`)
      (`PrimitiveComponent.SetCollisionObjectType` _collisioncomponent "ECC_GameTraceChannel3")
      (`MaterialInstanceDynamic.SetVectorParameterValue` _setballcolor "ballColor" (`self.greenColor`))
      (bind _asmy_character_3 (cast `/Game/Blueprints/MyCharacter` _returnvalue))
      (set `/Game/Blueprints/MyCharacter.myBallColor` "NewEnumerator1" _asmy_character_3)
      (goto _label)
      (elif (`self.isBlue`)
        (`PrimitiveComponent.SetCollisionObjectType` _collisioncomponent "ECC_GameTraceChannel2")
        (`MaterialInstanceDynamic.SetVectorParameterValue` _setballcolor "ballColor" (`self.blueColor`))
        (bind _asmy_character_4 (cast `/Game/Blueprints/MyCharacter` _returnvalue))
        (set `/Game/Blueprints/MyCharacter.myBallColor` "NewEnumerator0" _asmy_character_4)
        (goto _label)))))

(fn `UserConstructionScript`
  (`SceneComponent.SetRelativeScale3D` (`self.colorChangingRing`) (`self.ringScale`))
  (bind _returnvalue (`PrimitiveComponent.CreateDynamicMaterialInstance` 0 "/Game/artSource/materials/colorChangingRing_mat.colorChangingRing_mat"))
  (set `self.colorShift` _returnvalue)
  (if (`self.isRed`)
    (`MaterialInstanceDynamic.SetVectorParameterValue` (`self.colorShift`) "baseColor" (`self.redColor`))
    (elif (`self.isGreen`)
      (`MaterialInstanceDynamic.SetVectorParameterValue` (`self.colorShift`) "baseColor" (`self.greenColor`))
      (elif (`self.isBlue`)
        (`MaterialInstanceDynamic.SetVectorParameterValue` (`self.colorShift`) "baseColor" (`self.blueColor`))))))