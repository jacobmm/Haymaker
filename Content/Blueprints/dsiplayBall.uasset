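; A colored ball actor with a projectile component, configured by its color type as normal (white), blue, green or red.
; The Construction Script applies the projectile's initial speed and creates a dynamic material instance on the sphere.
; A switch on the color type sets the material's color parameter and gives the collision component a separate custom object channel per color.
; BeginPlay is empty, so the graphs add no runtime logic.
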(event `self.ReceiveBeginPlay`)

(fn `UserConstructionScript`
  (bind _collisioncomponent (`self.CollisionComponent`))
  (set `ProjectileMovementComponent.InitialSpeed` (`self.projectileSpeed`) (`self.Projectile`))
  (bind _returnvalue (`PrimitiveComponent.CreateDynamicMaterialInstance` (`self.Sphere`) 0 "/Game/artSource/materials/ball_Inst.ball_Inst"))
  (set `self.setBallColor` _returnvalue)
  (switch `/Game/Blueprints/tools/ballColor` (`self.myColor`)
    (:`NewEnumerator0`
      (`PrimitiveComponent.SetCollisionObjectType` _collisioncomponent "ECC_GameTraceChannel2")
      (`MaterialInstanceDynamic.SetVectorParameterValue` (`self.setBallColor`) "ballColor" (`self.blueColor`)))
    (:`NewEnumerator1`
      (`PrimitiveComponent.SetCollisionObjectType` _collisioncomponent "ECC_GameTraceChannel3")
      (`MaterialInstanceDynamic.SetVectorParameterValue` (`self.setBallColor`) "ballColor" (`self.greenColor`)))
    (:`NewEnumerator2`
      (`PrimitiveComponent.SetCollisionObjectType` _collisioncomponent "ECC_GameTraceChannel1")
      (`MaterialInstanceDynamic.SetVectorParameterValue` (`self.setBallColor`) "ballColor" (`self.whiteColor`)))
    (:`NewEnumerator3`
      (`PrimitiveComponent.SetCollisionObjectType` _collisioncomponent "ECC_GameTraceChannel4")
      (`MaterialInstanceDynamic.SetVectorParameterValue` (`self.setBallColor`) "ballColor" (`self.redColor`)))))