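; Laser field hazard that reacts to projectiles and characters entering its Laserbox.
; On overlap, it casts the other actor to MyProjectile or MyCharacter, then routes both through shared equality checks.
; A projectile triggers ReturnBallMessage on player controller 0's pawn.
; A character dies via Death unless its LerpPort flag is set, so characters in that state pass unharmed.
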(event `self.laserbox.OnComponentBeginOverlap`
  (params (OtherActor :type "Actor Object Reference") (OtherComp :type "PrimitiveComponent Object Reference") (OtherBodyIndex :type Integer) (bFromSweep :type Boolean) (SweepResult :type "HitResult Structure (by ref)"))
  (bind _asmy_projectile (cast `/Game/Blueprints/MyProjectile` OtherActor)
    (:`then`
      _)
    (:`CastFailed`
      (bind _asmy_character (cast `/Game/Blueprints/MyCharacter` OtherActor))))
  (if (== _asmy_projectile OtherActor)
    (message `/Game/Blueprints/haymkaerBP/playerInteraction_BPI.returnBall` (`Controller.K2_GetPawn` (`GameplayStatics.GetPlayerController` 0)))
    (elif (== _asmy_character OtherActor)
      (bind _asmy_character_2 (cast `/Game/Blueprints/MyCharacter` OtherActor))
      (if (not (`/Game/Blueprints/MyCharacter.lerpPort` _asmy_character_2))
        (`/Game/Blueprints/MyCharacter.death` _asmy_character_2)))))

(fn `UserConstructionScript`)