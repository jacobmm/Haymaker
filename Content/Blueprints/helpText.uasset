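; Help text actor that shows a hint on screen and marks its location with a fire effect through two trigger volumes.
; BeginPlay creates a HelpTextWidget from HelpTextInfo, which TextTrigger adds to and removes from the viewport on overlap begin and end.
; NoticeTrigger spawns a P_Fire emitter at the actor and destroys it on overlap end, without filtering the overlapping actor.
; The updateText event swaps the widget's string to HelpTextInfo2.
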(event `self.ReceiveBeginPlay`
  (bind _returnvalue (`|CreateWidget` "/Game/Blueprints/umg/helpTextWidget.helpTextWidget_C" (`GameplayStatics.GetPlayerController` 0) (`self.helpTextInfo`)))
  (set `self.helpTextWidget` _returnvalue))

(event `self.ReceiveActorBeginOverlap`
  (params (OtherActor :type "Actor Object Reference")))

(event `self.ReceiveTick`
  (params (DeltaSeconds :type "Float (single-precision)")))

(event `updateText`
  (set `/Game/Blueprints/umg/helpTextWidget.helpTextString` (`self.HelpTextInfo2`) (`self.helpTextWidget`)))

(event `self.textTrigger.OnComponentBeginOverlap`
  (params (OtherActor :type "Actor Object Reference") (OtherComp :type "PrimitiveComponent Object Reference") (OtherBodyIndex :type Integer) (bFromSweep :type Boolean) (SweepResult :type "HitResult Structure (by ref)"))
  (`UserWidget.AddToViewport` (`self.helpTextWidget`) 0))

(event `self.textTrigger.OnComponentEndOverlap`
  (params (OtherActor :type "Actor Object Reference") (OtherComp :type "PrimitiveComponent Object Reference") (OtherBodyIndex :type Integer))
  (`Widget.RemoveFromParent` (`self.helpTextWidget`)))

(event `self.noticeTrigger.OnComponentBeginOverlap`
  (params (OtherActor :type "Actor Object Reference") (OtherComp :type "PrimitiveComponent Object Reference") (OtherBodyIndex :type Integer) (bFromSweep :type Boolean) (SweepResult :type "HitResult Structure (by ref)"))
  (bind _returnvalue (`GameplayStatics.SpawnEmitterAtLocation` "/Game/StarterContent/Particles/P_Fire.P_Fire" (`self.K2_GetActorLocation`) (struct) false)))

(event `self.noticeTrigger.OnComponentEndOverlap`
  (params (OtherActor :type "Actor Object Reference") (OtherComp :type "PrimitiveComponent Object Reference") (OtherBodyIndex :type Integer))
  (`ActorComponent.K2_DestroyComponent` (stale `self.noticeTrigger.OnComponentBeginOverlap` _returnvalue)))

(fn `UserConstructionScript`)