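; Moving colored force field that slides and rotates like a door, started on spawn or by a MyCharacter entering its trigger.
; A timeline lerps the mesh to an end position and rotation, then reverses after a delay, or locks if single-use.
; Leaving the trigger reverses reusable fields.
; Construction script sizes trigger and mesh, previews the end pose, and sets a color-specific collision profile and dynamic material.
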(event `self.ReceiveBeginPlay`
  (bind _onetimeuse (`self.oneTimeUse`))
  ;[1 1 1] Movement timing
  (`TimelineComponent.SetPlayRate` (`self.doorTimeline`) (/ 1.0 (`self.travelTimeInSeconds`)))
  (if (`self.startOnSpawn`)
    ;[1 1 1] Movement of the feild
    (bind (_direction _lerp_position_alpha _lerp_rotation_alpha) (`Timeline|doorTimeline` :!via `PlayFromStart` :!label _label)
      (:`Update`
        (`SceneComponent.K2_SetRelativeLocationAndRotation` (`self.feildMesh`) (`KismetMathLibrary.VLerp` (`self.DoorLocation`) (`self.endPosition`) _lerp_position_alpha) (`KismetMathLibrary.RLerp` (struct) (`self.rotationScale`) _lerp_rotation_alpha) false))
      (:`Finished`
        (`KismetSystemLibrary.RetriggerableDelay` (`self.StopDelay`))
        (switch `ETimelineDirection` _direction
          (:`Forward`
            (if _onetimeuse
              (set `self.locked` true)
              (else
                (`self.backward`))))
          (:`Backward`
            (if _onetimeuse
              (set `self.locked` true)
              (else
                (`self.forward`)))))))))

(event `self.doorTrigger.OnComponentBeginOverlap`
  (params (OtherActor :type "Actor Object Reference") (OtherComp :type "PrimitiveComponent Object Reference") (OtherBodyIndex :type Integer) (bFromSweep :type Boolean) (SweepResult :type "HitResult Structure (by ref)"))
  ;[1 1 1] Movement of the feild
  (bind _asmy_character (cast `/Game/Blueprints/MyCharacter` OtherActor))
  (if (== _asmy_character OtherActor)
    (if (not (`self.locked`))
      (goto _label :!via `PlayFromStart`))))

(event `forward`
  ;[1 1 1] Movement of the feild
  (goto _label :!via `PlayFromStart`))

(event `self.doorTrigger.OnComponentEndOverlap`
  (params (OtherActor :type "Actor Object Reference") (OtherComp :type "PrimitiveComponent Object Reference") (OtherBodyIndex :type Integer))
  ;[1 1 1] Movement of the feild
  (bind _asmy_character (cast `/Game/Blueprints/MyCharacter` OtherActor))
  (if (and (== _asmy_character OtherActor) (!= (`self.oneTimeUse`) true))
    (goto _label :!via `ReverseFromEnd`)))

(event `backward`
  ;[1 1 1] Movement of the feild
  (goto _label :!via `ReverseFromEnd`))

(fn `UserConstructionScript`
  (bind _feildmesh (`self.feildMesh`))
  (bind _feildmesh_2 (`self.feildMesh`))
  (bind _doortrigger (`self.doorTrigger`))
  (bind _triggerscale (`self.TriggerScale`))
  (bind _forcefield_mi (`self.forcefield MI`))
  (bind _returnvalue (`PrimitiveComponent.CreateDynamicMaterialInstance` (`self.feildMesh`) 0 "/Game/artSource/materials/forceField.forceField"))
  (set `self.forcefield MI` _returnvalue)
  ;[1 1 1] trigger size and location (Z scales up from the ground.)
  (`SceneComponent.SetRelativeScale3D` _doortrigger _triggerscale)
  (`SceneComponent.K2_SetRelativeLocation` _doortrigger (`KismetMathLibrary.MakeVector` (.x (`self.TriggerLocation`)) (.y (`self.TriggerLocation`)) (+ (.z (`self.TriggerLocation`)) (/ (* (.z _triggerscale) 60.0) 2.0))) false)
  ;[1 1 1] rotation
  (set `self.rotationScale` (`KismetMathLibrary.MakeRot` (`self.EndPitch`) (`self.EndYaw`) (`self.EndRoll`)))
  ;[1 1 1] Door location and scale
  (`SceneComponent.K2_SetRelativeLocation` _feildmesh_2 (`self.DoorLocation`) false)
  (`SceneComponent.SetRelativeScale3D` _feildmesh_2 (`self.DoorScale`))
  ;[1 1 1] test end position and rotation
  (`SceneComponent.K2_SetRelativeLocationAndRotation` (`self.feildMesh`) (`KismetMathLibrary.SelectVector` (`self.endPosition`) (`self.DoorLocation`) (`self.testEndPostion`)) (`KismetMathLibrary.SelectRotator` (`self.rotationScale`) (struct) (`self.TestEndRotation`)) false)
  ;[1 1 1] set wall color
  (switch `/Game/Blueprints/tools/fieldColor` (`self.myColor`)
    (:`NewEnumerator0`
      (`PrimitiveComponent.SetCollisionProfileName` _feildmesh "blueWall")
      (`MaterialInstanceDynamic.SetVectorParameterValue` _forcefield_mi "wallColor" (`self.blueWall`)))
    (:`NewEnumerator2`
      (`PrimitiveComponent.SetCollisionProfileName` _feildmesh "greenWall")
      (`MaterialInstanceDynamic.SetVectorParameterValue` _forcefield_mi "wallColor" (`self.greenWall`)))
    (:`NewEnumerator3`
      (`PrimitiveComponent.SetCollisionProfileName` _feildmesh "redWall")
      (`MaterialInstanceDynamic.SetVectorParameterValue` _forcefield_mi "wallColor" (`self.redWall`)))))