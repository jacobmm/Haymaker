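; Golf pawn that handles look input and a fire action keyed to the selected club type.
; Turn and LookUp axes drive controller yaw and pitch, while Fire switches on ClubType but only prints the club name in every case.
; PitchInfoRPC smooths AimPitchInfo toward player 0's control-minus-pawn rotation pitch using RInterpTo.
; The serverTurn event and construction script are empty stubs.
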(event `serverTurn`)

(event `InputAxis|Turn` :overrideparent false
  (params (AxisValue :type "Float (single-precision)"))
  ;[1 1 1] look
  (`self.AddControllerYawInput` AxisValue))

(event `InputAxis|LookUp` :overrideparent false
  (params (AxisValue :type "Float (single-precision)"))
  ;[1 1 1] look
  (`self.AddControllerPitchInput` AxisValue))

(event `InputAction|Fire`
  (params (Key :type "Key Structure" :default "AnyKey"))
  (bind _clubtype (`self.clubType`))
  (bind _returnvalue (`|GetEnumeratorNameAsString` _clubtype))
  ;[1 1 1] shoot
  (:`Pressed`
    (switch `/Game/Blueprints/haymkaerBP/E_clubType` _clubtype
      (:`NewEnumerator0`
        (`KismetSystemLibrary.PrintString` _returnvalue))
      (:`NewEnumerator1`
        (`KismetSystemLibrary.PrintString` _returnvalue))
      (:`NewEnumerator2`
        (`KismetSystemLibrary.PrintString` _returnvalue))
      (:`NewEnumerator3`
        (`KismetSystemLibrary.PrintString` _returnvalue))
      (:`NewEnumerator4`
        (`KismetSystemLibrary.PrintString` _returnvalue)))))

(fn `pitchInfoRPC`
  (returns (outPitch :type "Float (double-precision)"))
  (bind _returnvalue (`GameplayStatics.GetPlayerController` 0))
  (bind _output_get (set `self.aimPitchInfo` (.pitch (`KismetMathLibrary.RInterpTo` (`KismetMathLibrary.MakeRotator` 0.0 (`self.aimPitchInfo`)) (`KismetMathLibrary.NormalizedDeltaRotator` (`Controller.GetControlRotation` _returnvalue) (`self.K2_GetActorRotation` (`Controller.K2_GetPawn` _returnvalue))) (`GameplayStatics.GetWorldDeltaSeconds`) 15.0))))
  (return _output_get))

(fn `UserConstructionScript`)