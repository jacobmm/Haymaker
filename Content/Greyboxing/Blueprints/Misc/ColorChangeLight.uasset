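; Greyboxing light actor that switches between two color and intensity presets each time it is activated.
; The construction script puts a dynamic Light_White material instance on the Bulb and applies the first preset to it and PointLight1.
; Activate calls ToggleColor, where a FlipFlop alternates presets, updating material and point light together, with material intensity scaled down from the light's value.
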(event `self.Activate`
  (`self.ToggleColor`))

(event `ToggleColor`
  (bind _pointlight1 (`self.PointLight1`))
  (bind _lightmaterial (`self.LightMaterial`))
  (`/Engine/EditorBlueprintResources/StandardMacros.FlipFlop`
    (:`A`
      ;[1 1 1] Update light material
      (`MaterialInstanceDynamic.SetVectorParameterValue` _lightmaterial "Color" (`self.Color2`))
      (`MaterialInstanceDynamic.SetScalarParameterValue` _lightmaterial "Intensity" (/ (`self.Intensity2`) 1000.0))
      ;[1 1 1] Update pointlight
      (`LightComponent.SetIntensity` _pointlight1 (`self.Intensity2`))
      (`LightComponent.SetLightColor` _pointlight1 (`self.Color2`)))
    (:`B`
      (`MaterialInstanceDynamic.SetVectorParameterValue` _lightmaterial "Color" (`self.Color1`))
      (`MaterialInstanceDynamic.SetScalarParameterValue` _lightmaterial "Intensity" (/ (`self.Intensity1`) 1000.0))
      (`LightComponent.SetIntensity` _pointlight1 (`self.Intensity1`))
      (`LightComponent.SetLightColor` _pointlight1 (`self.Color1`)))))

(fn `UserConstructionScript`
  (bind _lightmaterial (`self.LightMaterial`))
  (bind _pointlight1 (`self.PointLight1`))
  (bind _returnvalue (`KismetMaterialLibrary.CreateDynamicMaterialInstance` "/Game/Greyboxing/Materials/Light_White.Light_White"))
  (set `self.LightMaterial` _returnvalue)
  (`PrimitiveComponent.SetMaterial` (`self.Bulb`) 0 (`self.LightMaterial`))
  (`MaterialInstanceDynamic.SetVectorParameterValue` _lightmaterial "Color" (`self.Color1`))
  (`MaterialInstanceDynamic.SetScalarParameterValue` _lightmaterial "Intensity" (/ (`self.Intensity1`) 1000.0))
  (`LightComponent.SetIntensity` _pointlight1 (`self.Intensity1`))
  (`LightComponent.SetLightColor` _pointlight1 (`self.Color1`)))